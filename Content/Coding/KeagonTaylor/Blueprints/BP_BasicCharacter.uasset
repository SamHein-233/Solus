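; Player character Blueprint that handles camera look, interaction crosshair feedback and the pause menu.
; Camera axes apply sensitivity and Y inversion, while a per-tick trace from the camera shows the crosshair only over actors implementing BP_Interact_Interface.
; BeginPlay adds the Enhanced Input context and creates both widgets.
; Menu, map and settings actions share one toggle that pauses the game and selects a WP_Menu switcher page.
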(event Input|EnhancedActionEvents|EnhancedInputActionIA_OpenMenu
  (params (ActionValue :type Boolean) (ElapsedSeconds :type Float%20%28double-precision%29) (TriggeredSeconds :type Float%20%28double-precision%29) (InputAction :type Input%20Action%20Object%20Reference :default "/Game/Coding/KeagonTaylor/Inputs/InputMaps/IA_OpenMenu.IA_OpenMenu"))
  (bind _returnvalue (Game|GetPlayerController 0))
  (bind _menu (Variables|Default|GetMenu))
  (bind (_sizex _sizey) (HUD|GetViewportSize _returnvalue))
  ;[1 1 1] Opening Menu (Keagon)
  (:Started
    (Variables|Default|SetWidgetID 0)
    (if (Variables|Default|GetMenuOpen)
      (Variables|Default|SetMenuOpen false)
      (Widget|RemovefromParent _menu)
      (Game|SetGamePaused false)
      (Input|SetInputModeGameOnly _returnvalue false)
      (Variables|/Script/Engine.PlayerController|SetbShowMouseCursor _returnvalue false)
      (else
        (Variables|Default|SetMenuOpen true)
        (Game|SetGamePaused true)
        (Utilities|FlowControl|Delay (Variables|Default|GetOpenDelay))
        (Class|WidgetSwitcher|SetActiveWidgetIndex (Variables|/Game/Coding/KeagonTaylor/Blueprints/Menus/WP_Menu.WP_Menu_C|GetWidgetSwitcher _menu) (Variables|Default|GetWidgetID))
        (UserInterface|Viewport|AddtoViewport _menu 0)
        (Variables|/Script/Engine.PlayerController|SetbShowMouseCursor _returnvalue true)
        (Class|PlayerController|SetMouseLocation _returnvalue (/ _sizex 2) (/ _sizey 2))))))

(event Input|EnhancedActionEvents|EnhancedInputActionIA_OpenMap
  (params (ActionValue :type Boolean) (ElapsedSeconds :type Float%20%28double-precision%29) (TriggeredSeconds :type Float%20%28double-precision%29) (InputAction :type Input%20Action%20Object%20Reference :default "/Game/Coding/KeagonTaylor/Inputs/InputMaps/IA_OpenMap.IA_OpenMap"))
  (bind _returnvalue (Game|GetPlayerController 0))
  (bind _menu (Variables|Default|GetMenu))
  (bind (_sizex _sizey) (HUD|GetViewportSize _returnvalue))
  ;[1 1 1] Opening Menu (Keagon)
  (:Started
    (Variables|Default|SetWidgetID 1)
    (if (Variables|Default|GetMenuOpen)
      (Variables|Default|SetMenuOpen false)
      (Widget|RemovefromParent _menu)
      (Game|SetGamePaused false)
      (Input|SetInputModeGameOnly _returnvalue false)
      (Variables|/Script/Engine.PlayerController|SetbShowMouseCursor _returnvalue false)
      (else
        (Variables|Default|SetMenuOpen true)
        (Game|SetGamePaused true)
        (Utilities|FlowControl|Delay (Variables|Default|GetOpenDelay))
        (Class|WidgetSwitcher|SetActiveWidgetIndex (Variables|/Game/Coding/KeagonTaylor/Blueprints/Menus/WP_Menu.WP_Menu_C|GetWidgetSwitcher _menu) (Variables|Default|GetWidgetID))
        (UserInterface|Viewport|AddtoViewport _menu 0)
        (Variables|/Script/Engine.PlayerController|SetbShowMouseCursor _returnvalue true)
        (Class|PlayerController|SetMouseLocation _returnvalue (/ _sizex 2) (/ _sizey 2))))))

(event Input|EnhancedActionEvents|EnhancedInputActionIA_OpenSettings
  (params (ActionValue :type Boolean) (ElapsedSeconds :type Float%20%28double-precision%29) (TriggeredSeconds :type Float%20%28double-precision%29) (InputAction :type Input%20Action%20Object%20Reference :default "/Game/Coding/KeagonTaylor/Inputs/InputMaps/IA_OpenSettings.IA_OpenSettings"))
  (bind _returnvalue (Game|GetPlayerController 0))
  (bind _menu (Variables|Default|GetMenu))
  (bind (_sizex _sizey) (HUD|GetViewportSize _returnvalue))
  ;[1 1 1] Opening Menu (Keagon)
  (:Started
    (Variables|Default|SetWidgetID 2)
    (if (Variables|Default|GetMenuOpen)
      (Variables|Default|SetMenuOpen false)
      (Widget|RemovefromParent _menu)
      (Game|SetGamePaused false)
      (Input|SetInputModeGameOnly _returnvalue false)
      (Variables|/Script/Engine.PlayerController|SetbShowMouseCursor _returnvalue false)
      (else
        (Variables|Default|SetMenuOpen true)
        (Game|SetGamePaused true)
        (Utilities|FlowControl|Delay (Variables|Default|GetOpenDelay))
        (Class|WidgetSwitcher|SetActiveWidgetIndex (Variables|/Game/Coding/KeagonTaylor/Blueprints/Menus/WP_Menu.WP_Menu_C|GetWidgetSwitcher _menu) (Variables|Default|GetWidgetID))
        (UserInterface|Viewport|AddtoViewport _menu 0)
        (Variables|/Script/Engine.PlayerController|SetbShowMouseCursor _returnvalue true)
        (Class|PlayerController|SetMouseLocation _returnvalue (/ _sizex 2) (/ _sizey 2))))))

(event EventBeginPlay
  (bind _returnvalue (Game|GetPlayerController 0))
  (bind _returnvalue_2 (PlayerController|LocalPlayerSubsystems|GetEnhancedInputLocalPlayerSubsystem _returnvalue))
  ;[1 1 1] Allow Custom Input (Keagon)
  (Utilities|FlowControl|Sequence
    (:then_0
      (Utilities|IsValid _returnvalue_2
        (:Is%20Valid
          (Input|AddMappingContext _returnvalue_2 "/Game/Coding/KeagonTaylor/Inputs/IMC_Basic.IMC_Basic" 0 "(bIgnoreAllPressedKeysUntilRelease=True,bForceImmediately=False)")
          (bind _returnvalue_3 (UserInterface|CreateWidget "/Game/Coding/KeagonTaylor/Blueprints/Menus/WP_Menu.WP_Menu_C"))
          (Variables|Default|SetMenu _returnvalue_3)
          (Input|EnableInput _returnvalue)
          (Variables|Default|SetOpenDelay 0.0))))
    (:then_1
      (bind _returnvalue_4 (UserInterface|CreateWidget "/Game/Coding/KeagonTaylor/Blueprints/W_Crosshair.W_Crosshair_C"))
      (Variables|Default|SetCrosshair _returnvalue_4))))

(event Collision|EventActorBeginOverlap
  (params (OtherActor :type Actor%20Object%20Reference)))

(event EventTick
  (params (DeltaSeconds :type Float%20%28single-precision%29))
  (bind _camera (Variables|Default|GetCamera))
  (bind _crosshair (Variables|Default|GetCrosshair))
  (bind _returnvalue (UserInterface|Viewport|IsinViewport _crosshair))
  (bind _returnvalue_2 (Transformation|GetWorldLocation _camera))
  ;[1 1 1] Crosshair detection (Keagon)
  (bind (_outhit _returnvalue_3) (Collision|LineTraceByChannel _returnvalue_2 (+ _returnvalue_2 (* (Math|Vector|GetForwardVector _camera) 5e+02)) "TraceTypeQuery1" false 0 "None"))
  (if _returnvalue_3
    (if (Utilities|DoesObjectImplementInterface (.HitActor (Collision|BreakHitResult _outhit)) "/Game/Coding/KeagonTaylor/Blueprints/BP_Interact_Interface.BP_Interact_Interface_C")
      (if (not _returnvalue)
        (UserInterface|Viewport|AddtoViewport _crosshair 0))
      (else
        (if _returnvalue :!label _label
          (Widget|RemovefromParent _crosshair))))
    (else
      (goto _label))))

(event Input|AxisEvents|InputAxisCameraY
  (params (AxisValue :type Float%20%28single-precision%29))
  ;[1 1 1] Camera (Ace)
  (Pawn|Input|AddControllerPitchInput (* AxisValue (Variables|Default|GetCamYInvertVal) (Variables|Default|GetCamYSensitivity))))

(event Input|AxisEvents|InputAxisCameraX
  (params (AxisValue :type Float%20%28single-precision%29))
  ;[1 1 1] Camera (Ace)
  (Pawn|Input|AddControllerYawInput (* AxisValue (Variables|Default|GetCamXSensitivity))))

(fn ConstructionScript)