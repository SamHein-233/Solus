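; BP_WireEnd is an interactable end point in a wire-matching puzzle, identified by its WireCount index.
; Its point light blinks from BeginPlay until that wire is marked complete in the BP_GameVariables game instance.
; On interaction it stores its index as TempEndWire and, if that matches TempStartWire, marks the wire complete.
; It then scans the completion array, setting WiresComplete once every entry through index 4 is true.
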(event EventBeginPlay
  (Rendering|SetVisibility (Variables|Default|GetPointLight) true false :!label _label)
  (Utilities|FlowControl|Delay 0.5)
  (Rendering|SetVisibility (Variables|Default|GetPointLight) false false)
  (Utilities|FlowControl|Delay 0.5)
  (bind _asbp_game_variables (Utilities|Casting|CastToBP_GameVariables (Game|GetGameInstance)))
  (if (Utilities|Array|Get(acopy) (Variables|/Game/Coding/Luke_Samuelson/BP_GameVariables.BP_GameVariables_C|GetWireComplete _asbp_game_variables) (Variables|Default|GetWire%20Count))
    (Rendering|Components|Light|SetLightFunctionMaterial (Variables|Default|GetPointLight) 0)
    (else
      (goto _label))))

(event EventInteractwithObject
  (bind _wire_count (Variables|Default|GetWire%20Count))
  (bind _asbp_game_variables (Utilities|Casting|CastToBP_GameVariables (Game|GetGameInstance)))
  (if (not (Variables|/Game/Coding/Luke_Samuelson/BP_GameVariables.BP_GameVariables_C|GetWiresComplete _asbp_game_variables))
    (Development|PrintString "Pressed")
    (bind _asbp_game_variables_2 (Utilities|Casting|CastToBP_GameVariables (Game|GetGameInstance))
      (:then
        (bind _output_get (Variables|/Game/Coding/Luke_Samuelson/BP_GameVariables.BP_GameVariables_C|SetTempEndWire _asbp_game_variables_2 _wire_count))
        (Math|Integer|CompareInt _output_get (Variables|/Game/Coding/Luke_Samuelson/BP_GameVariables.BP_GameVariables_C|GetTempStartWire _asbp_game_variables_2)
          (:==
            (Utilities|Array|SetArrayElem (Variables|/Game/Coding/Luke_Samuelson/BP_GameVariables.BP_GameVariables_C|GetWireComplete _asbp_game_variables_2) _wire_count true)
            (bind (_array_element _array_index) (Utilities|Array|ForEachLoopwithBreak (Variables|/Game/Coding/Luke_Samuelson/BP_GameVariables.BP_GameVariables_C|GetWireComplete _asbp_game_variables_2) :!label _label)
              (:LoopBody
                (if _array_element
                  (Math|Integer|CompareInt _array_index 4
                    (:==
                      (bind _asbp_game_variables_3 (Utilities|Casting|CastToBP_GameVariables (Game|GetGameInstance)))
                      (Variables|/Game/Coding/Luke_Samuelson/BP_GameVariables.BP_GameVariables_C|SetWiresComplete _asbp_game_variables_3 true)
                      (Development|PrintString "Wires Compelte")))
                  (else
                    (goto _label Break))))))))
      (:CastFailed
        (Development|PrintString "Button Cast Failed")))))

(fn ConstructionScript
  (|CallParentFunction))