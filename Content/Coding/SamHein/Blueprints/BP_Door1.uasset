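; BP_Door1 is a key-locked sliding door that reacts when the first-person character enters its sphere collision.
; If the character has a key, a timeline slides the door along its local Y axis; otherwise a no-access widget shows and all widgets are cleared after a delay.
; End overlap is wired to clear the key and widget, but first casts the same actor to both character and BP_Door.
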(event OnComponentBeginOverlap(SphereCollision)
  (params (OverlappedComponent :type Primitive%20Component%20Object%20Reference) (OtherActor :type Actor%20Object%20Reference) (OtherComp :type Primitive%20Component%20Object%20Reference) (OtherBodyIndex :type Integer) (bFromSweep :type Boolean) (SweepResult :type Hit%20Result%20Structure%20%28by%20ref%29))
  (bind _asbp_first_person_character (Utilities|Casting|CastToBP_FirstPersonCharacter OtherActor))
  (if (Variables|/Game/Coding/Derek_Scheuerman/FirstPerson/Blueprints/BP_FirstPersonCharacter.BP_FirstPersonCharacter_C|GetHasKey? _asbp_first_person_character)
    (bind _newtrack_0 (Timeline|Timeline Play)
      (:Update
        (Transformation|SetRelativeLocation (Variables|Default|GetDoor) (Math|Vector|MakeVector 0.0 (* _newtrack_0 1.9e+02) 0.0) false false)))
    (else
      (bind _returnvalue (UserInterface|CreateWidget "/Game/Coding/SamHein/Widgets/W_NoAccess.W_NoAccess_C"))
      (bind _output_get (Variables|Default|SetNoAccess _returnvalue))
      (UserInterface|Viewport|AddtoViewport _output_get 0)
      (Utilities|FlowControl|Delay 3.0)
      (Viewport|RemoveAllWidgets))))

(event OnComponentEndOverlap(SphereCollision)
  (params (OverlappedComponent :type Primitive%20Component%20Object%20Reference) (OtherActor :type Actor%20Object%20Reference) (OtherComp :type Primitive%20Component%20Object%20Reference) (OtherBodyIndex :type Integer))
  (bind _asbp_first_person_character (Utilities|Casting|CastToBP_FirstPersonCharacter OtherActor))
  (Utilities|Casting|CastToBP_Door OtherActor)
  (Variables|/Game/Coding/Derek_Scheuerman/FirstPerson/Blueprints/BP_FirstPersonCharacter.BP_FirstPersonCharacter_C|SetHasKey? _asbp_first_person_character false)
  (Widget|RemovefromParent (Variables|Default|GetNoAccess)))

(fn ConstructionScript)