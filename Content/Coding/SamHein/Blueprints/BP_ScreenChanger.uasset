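; BP_ScreenChanger is an interactable screen that turns on and plays a cinematic.
; InteractwithObject swaps the Screen material to the on state, hides the ACE player character and plays the Level Sequence.
; A fixed delay, rather than a sequence-finished event, times when the player reappears and a 2D music sound is spawned, stored and played.
; Nothing guards against repeat interaction, as the branch condition is always true.
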(event EventInteractwithObject
  (if true
    (Rendering|Material|SetMaterial (Variables|Default|GetScreen) 0 "/Game/Coding/SamHein/MI_ScreenOn.MI_ScreenOn")
    (bind _asbp_player_character_ace (Utilities|Casting|CastToBP_PlayerCharacterACE (Game|GetPlayerCharacter 0)))
    (Rendering|SetActorHiddenInGame _asbp_player_character_ace true)
    (Sequencer|Player|Play (Variables|/Script/LevelSequence.LevelSequenceActor|GetSequencePlayer (Variables|Default|GetLevel%20Sequence)) :!class /Script/MovieScene.MovieSceneSequencePlayer)
    (Utilities|FlowControl|Delay 27.6)
    (Rendering|SetActorHiddenInGame _asbp_player_character_ace false)
    (bind _returnvalue (Audio|SpawnSound2D (Variables|Default|GetMusic) 1.0 1.0 0.0 0))
    (bind _output_get (Variables|Default|SetMusicRef _returnvalue))
    (Audio|Components|Audio|Play _output_get 0.0)))

(fn ConstructionScript
  (|CallParentFunction))