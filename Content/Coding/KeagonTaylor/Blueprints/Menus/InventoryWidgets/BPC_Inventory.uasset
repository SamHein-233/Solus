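; Inventory component that stores item names and descriptions and passes a selected item to the menu widget.
; On BeginPlay it creates and keeps references to the log and menu widgets, without adding either to the viewport here.
; AddItem appends to parallel name and description arrays and prints the new name and index.
; SwapItem looks up both arrays by item ID and forwards the entry to the menu widget.
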(event EventBeginPlay
  (bind _returnvalue (UserInterface|CreateWidget "/Game/Coding/KeagonTaylor/Blueprints/Menus/WP_Log.WP_Log_C"))
  (Variables|Default|SetW_Log _returnvalue)
  (bind _returnvalue_2 (UserInterface|CreateWidget "/Game/Coding/KeagonTaylor/Blueprints/Menus/WP_Menu.WP_Menu_C"))
  (Variables|Default|SetW_Menu _returnvalue_2))

(fn AddItem
  (params (ItemName :type Text) (ItemDescription :type Text))
  (bind _itemnamearray (Variables|Default|GetItemNameArray))
  (bind _returnvalue (Utilities|Array|Add _itemnamearray ItemName))
  (Development|PrintText (Utilities|Array|Get(acopy) _itemnamearray _returnvalue))
  (Development|PrintText (Utilities|Text|ToText(Integer) _returnvalue))
  (Utilities|Array|Add (Variables|Default|GetItemDescriptionArray) ItemDescription))

(fn SwapItem
  (params (ItemID :type Integer))
  (Default|SwapItem (Variables|Default|GetW_Menu) (Utilities|Array|Get(acopy) (Variables|Default|GetItemNameArray) ItemID) (Utilities|Array|Get(acopy) (Variables|Default|GetItemDescriptionArray) ItemID)))