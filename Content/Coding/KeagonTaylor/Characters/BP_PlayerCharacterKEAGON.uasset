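; Player character Blueprint handling movement, jumping, camera look and the player's menu screens.
; Enhanced Input actions toggle a game-pausing tabbed menu opened at the menu, map or settings page, plus a separate pause menu, switching cursor and input mode.
; Legacy axis and key events drive controls, gated by an IsMenuClosed macro, with a debug forward-speed toggle.
; A WIP sensitivity menu sits on a debug key; the interactable crosshair trace is disconnected.
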(event Custom|ResumePressed
  (bind _returnvalue (Game|GetPlayerController 0))
  (bind _pausemenu (Variables|Default|GetPauseMenu))
  (Development|PrintString "CharacterResumePressed")
  (if (Variables|Default|GetPauseOpen)
    (Variables|Default|SetPauseOpen false)
    (Widget|RemovefromParent _pausemenu)
    (Game|SetGamePaused false)
    (Input|SetInputModeGameOnly _returnvalue false)
    (Variables|/Script/Engine.PlayerController|SetbShowMouseCursor _returnvalue false)
    (else
      (Variables|Default|SetPauseOpen true)
      (UserInterface|Viewport|AddtoViewport _pausemenu 0)
      (Game|SetGamePaused true)
      (Input|SetInputModeGameandUI _returnvalue _pausemenu "DoNotLock" false false)
      (Variables|/Script/Engine.PlayerController|SetbShowMouseCursor _returnvalue true))))

(event Input|EnhancedActionEvents|EnhancedInputActionIA_OpenPause
  (params (ActionValue :type Boolean) (ElapsedSeconds :type Float%20%28double-precision%29) (TriggeredSeconds :type Float%20%28double-precision%29) (InputAction :type Input%20Action%20Object%20Reference :default "/Game/Coding/KeagonTaylor/Inputs/InputMaps/IA_OpenPause.IA_OpenPause"))
  (bind _returnvalue (Game|GetPlayerController 0))
  (bind _pausemenu (Variables|Default|GetPauseMenu))
  (:Started
    (if (Variables|Default|GetProcessing) :!label _label
      (Utilities|FlowControl|Delay 0.5)
      (goto _label)
      (else
        (if (Variables|Default|GetSaveDisabled)
          (Development|PrintText "Save Disabled"))
        (if (Variables|Default|GetPauseOpen)
          (Variables|Default|SetPauseOpen false)
          (Widget|RemovefromParent _pausemenu)
          (Game|SetGamePaused false)
          (Input|SetInputModeGameOnly _returnvalue false)
          (Variables|/Script/Engine.PlayerController|SetbShowMouseCursor _returnvalue false)
          (else
            (Variables|Default|SetPauseOpen true)
            (UserInterface|Viewport|AddtoViewport _pausemenu 0)
            (Game|SetGamePaused true)
            (Input|SetInputModeGameandUI _returnvalue _pausemenu "DoNotLock" false false)
            (Variables|/Script/Engine.PlayerController|SetbShowMouseCursor _returnvalue true)))))))

(event Input|EnhancedActionEvents|EnhancedInputActionIA_OpenMenu
  (params (ActionValue :type Boolean) (ElapsedSeconds :type Float%20%28double-precision%29) (TriggeredSeconds :type Float%20%28double-precision%29) (InputAction :type Input%20Action%20Object%20Reference :default "/Game/Coding/KeagonTaylor/Inputs/InputMaps/IA_OpenMenu.IA_OpenMenu"))
  (bind _returnvalue (Game|GetPlayerController 0))
  (bind _menu (Variables|Default|GetMenu))
  (bind (_sizex _sizey) (HUD|GetViewportSize _returnvalue))
  ;[1 0.3961 0.702] Opening Menu (Keagon)
  (:Started
    (Variables|Default|SetWidgetID 0)
    (if (not (Variables|Default|GetProcessing))
      (Variables|Default|SetProcessing true)
      (if (Variables|Default|GetMenuOpen)
        (Variables|/Script/Engine.PlayerController|SetbShowMouseCursor _returnvalue false)
        (Input|SetInputModeGameOnly _returnvalue false)
        (Widget|RemovefromParent _menu)
        (Game|SetGamePaused false)
        (Utilities|FlowControl|Delay (Variables|Default|GetCloseDelay))
        (Variables|Default|SetMenuOpen false)
        (Variables|Default|SetProcessing false)
        (Class|Image|SetOpacity (Variables|/Game/Coding/KeagonTaylor/Blueprints/W_Crosshair.W_Crosshair_C|GetCrosshair_Dot (Variables|Default|GetCrosshair)) 1.0)
        (else
          (Class|Image|SetOpacity (Variables|/Game/Coding/KeagonTaylor/Blueprints/W_Crosshair.W_Crosshair_C|GetCrosshair_Dot (Variables|Default|GetCrosshair)) 0.0)
          (Variables|Default|SetMenuOpen true)
          (Utilities|FlowControl|Delay (Variables|Default|GetOpenDelay))
          (Game|SetGamePaused true)
          (Class|WidgetSwitcher|SetActiveWidgetIndex (Variables|/Game/Coding/KeagonTaylor/Blueprints/Menus/WP_Menu.WP_Menu_C|GetWidgetSwitcher _menu) (Variables|Default|GetWidgetID))
          (UserInterface|Viewport|AddtoViewport _menu 0)
          (Variables|/Script/Engine.PlayerController|SetbShowMouseCursor _returnvalue true)
          (Class|PlayerController|SetMouseLocation _returnvalue (/ _sizex 2) (/ _sizey 2))
          (Input|SetInputModeGameandUI _returnvalue _menu "DoNotLock" true false)
          (Variables|Default|SetProcessing false))))))

(event Input|EnhancedActionEvents|EnhancedInputActionIA_OpenMap
  (params (ActionValue :type Boolean) (ElapsedSeconds :type Float%20%28double-precision%29) (TriggeredSeconds :type Float%20%28double-precision%29) (InputAction :type Input%20Action%20Object%20Reference :default "/Game/Coding/KeagonTaylor/Inputs/InputMaps/IA_OpenMap.IA_OpenMap"))
  (bind _returnvalue (Game|GetPlayerController 0))
  (bind _menu (Variables|Default|GetMenu))
  (bind (_sizex _sizey) (HUD|GetViewportSize _returnvalue))
  ;[1 0.3961 0.702] Opening Menu (Keagon)
  (:Started
    (Variables|Default|SetWidgetID 1)
    (if (not (Variables|Default|GetProcessing))
      (Variables|Default|SetProcessing true)
      (if (Variables|Default|GetMenuOpen)
        (Variables|/Script/Engine.PlayerController|SetbShowMouseCursor _returnvalue false)
        (Input|SetInputModeGameOnly _returnvalue false)
        (Widget|RemovefromParent _menu)
        (Game|SetGamePaused false)
        (Utilities|FlowControl|Delay (Variables|Default|GetCloseDelay))
        (Variables|Default|SetMenuOpen false)
        (Variables|Default|SetProcessing false)
        (Class|Image|SetOpacity (Variables|/Game/Coding/KeagonTaylor/Blueprints/W_Crosshair.W_Crosshair_C|GetCrosshair_Dot (Variables|Default|GetCrosshair)) 1.0)
        (else
          (Class|Image|SetOpacity (Variables|/Game/Coding/KeagonTaylor/Blueprints/W_Crosshair.W_Crosshair_C|GetCrosshair_Dot (Variables|Default|GetCrosshair)) 0.0)
          (Variables|Default|SetMenuOpen true)
          (Utilities|FlowControl|Delay (Variables|Default|GetOpenDelay))
          (Game|SetGamePaused true)
          (Class|WidgetSwitcher|SetActiveWidgetIndex (Variables|/Game/Coding/KeagonTaylor/Blueprints/Menus/WP_Menu.WP_Menu_C|GetWidgetSwitcher _menu) (Variables|Default|GetWidgetID))
          (UserInterface|Viewport|AddtoViewport _menu 0)
          (Variables|/Script/Engine.PlayerController|SetbShowMouseCursor _returnvalue true)
          (Class|PlayerController|SetMouseLocation _returnvalue (/ _sizex 2) (/ _sizey 2))
          (Input|SetInputModeGameandUI _returnvalue _menu "DoNotLock" true false)
          (Variables|Default|SetProcessing false))))))

(event Input|EnhancedActionEvents|EnhancedInputActionIA_OpenSettings
  (params (ActionValue :type Boolean) (ElapsedSeconds :type Float%20%28double-precision%29) (TriggeredSeconds :type Float%20%28double-precision%29) (InputAction :type Input%20Action%20Object%20Reference :default "/Game/Coding/KeagonTaylor/Inputs/InputMaps/IA_OpenSettings.IA_OpenSettings"))
  (bind _returnvalue (Game|GetPlayerController 0))
  (bind _menu (Variables|Default|GetMenu))
  (bind (_sizex _sizey) (HUD|GetViewportSize _returnvalue))
  ;[1 0.3961 0.702] Opening Menu (Keagon)
  (:Started
    (Variables|Default|SetWidgetID 2)
    (if (not (Variables|Default|GetProcessing))
      (Variables|Default|SetProcessing true)
      (if (Variables|Default|GetMenuOpen)
        (Variables|/Script/Engine.PlayerController|SetbShowMouseCursor _returnvalue false)
        (Input|SetInputModeGameOnly _returnvalue false)
        (Widget|RemovefromParent _menu)
        (Game|SetGamePaused false)
        (Utilities|FlowControl|Delay (Variables|Default|GetCloseDelay))
        (Variables|Default|SetMenuOpen false)
        (Variables|Default|SetProcessing false)
        (Class|Image|SetOpacity (Variables|/Game/Coding/KeagonTaylor/Blueprints/W_Crosshair.W_Crosshair_C|GetCrosshair_Dot (Variables|Default|GetCrosshair)) 1.0)
        (else
          (Class|Image|SetOpacity (Variables|/Game/Coding/KeagonTaylor/Blueprints/W_Crosshair.W_Crosshair_C|GetCrosshair_Dot (Variables|Default|GetCrosshair)) 0.0)
          (Variables|Default|SetMenuOpen true)
          (Utilities|FlowControl|Delay (Variables|Default|GetOpenDelay))
          (Game|SetGamePaused true)
          (Class|WidgetSwitcher|SetActiveWidgetIndex (Variables|/Game/Coding/KeagonTaylor/Blueprints/Menus/WP_Menu.WP_Menu_C|GetWidgetSwitcher _menu) (Variables|Default|GetWidgetID))
          (UserInterface|Viewport|AddtoViewport _menu 0)
          (Variables|/Script/Engine.PlayerController|SetbShowMouseCursor _returnvalue true)
          (Class|PlayerController|SetMouseLocation _returnvalue (/ _sizex 2) (/ _sizey 2))
          (Input|SetInputModeGameandUI _returnvalue _menu "DoNotLock" true false)
          (Variables|Default|SetProcessing false))))))

(event EventBeginPlay
  (bind _returnvalue (Game|GetPlayerController 0))
  (bind _returnvalue_2 (PlayerController|LocalPlayerSubsystems|GetEnhancedInputLocalPlayerSubsystem _returnvalue))
  ;[1 1 1] CamYInvert (Ace)
  (Utilities|FlowControl|Sequence
    (:then_0
      (if (Variables|Default|GetCamYInvert)
        (Variables|Default|SetCamYInvertVal -1)
        (else
          (Variables|Default|SetCamYInvertVal 1))))
    (:then_1
      ;[1 0.3961 0.702] Menu Setup (Keagon)
      (bind _returnvalue_3 (UserInterface|CreateWidget "/Game/Coding/KeagonTaylor/Blueprints/W_Crosshair.W_Crosshair_C"))
      (bind _output_get (Variables|Default|SetCrosshair _returnvalue_3))
      (UserInterface|Viewport|AddtoViewport _output_get 0)
      (Utilities|IsValid _returnvalue_2
        (:Is%20Valid
          (Input|AddMappingContext _returnvalue_2 "/Game/Coding/KeagonTaylor/Inputs/IMC_Basic.IMC_Basic" 0 "(bIgnoreAllPressedKeysUntilRelease=True,bForceImmediately=False)")
          (bind _returnvalue_4 (UserInterface|CreateWidget "/Game/Coding/KeagonTaylor/Blueprints/Menus/WP_Menu.WP_Menu_C"))
          (Variables|Default|SetMenu _returnvalue_4)
          (Input|EnableInput _returnvalue)
          (Variables|Default|SetOpenDelay 0.0)
          (Variables|Default|SetMenuOpen false)
          (Variables|Default|SetCloseDelay 0.0))))
    (:then_2
      (bind _returnvalue_5 (UserInterface|CreateWidget "/Game/Coding/KeagonTaylor/Blueprints/Menus/WP_Tasks.WP_Tasks_C"))
      (Variables|Default|SetTasksMenu _returnvalue_5)
      (bind _returnvalue_6 (UserInterface|CreateWidget "/Game/Coding/KeagonTaylor/Blueprints/Menus/W_PauseMenu.W_PauseMenu_C"))
      (Variables|Default|SetPauseMenu _returnvalue_6))))

(event EventTick
  (params (DeltaSeconds :type Float%20%28single-precision%29))
  ;[1 0.3961 0.702] Crosshair detection (Keagon)
)

(event Input|AxisEvents|InputAxisForwardBack
  (params (AxisValue :type Float%20%28single-precision%29))
  ;[1 1 1] WASD Movement (Ace)
  (Utilities|IsMenuClosed
    (:then
      (Pawn|Input|AddMovementInput (Transformation|GetActorForwardVector) (* (Variables|Default|GetMaxSpeed) AxisValue) false))))

(event Input|AxisEvents|InputAxisLeftRight
  (params (AxisValue :type Float%20%28single-precision%29))
  ;[1 1 1] WASD Movement (Ace)
  (Utilities|IsMenuClosed
    (:then
      (Pawn|Input|AddMovementInput (Transformation|GetActorRightVector) AxisValue false))))

(event Input|AxisEvents|InputAxisCameraY
  (params (AxisValue :type Float%20%28single-precision%29))
  ;[1 1 1] Camera (Ace)
  (Utilities|IsMenuClosed
    (:then
      (Pawn|Input|AddControllerPitchInput (* AxisValue (Variables|Default|GetCamYInvertVal) (Variables|Default|GetCamYSensitivity))))))

(event Input|AxisEvents|InputAxisCameraX
  (params (AxisValue :type Float%20%28single-precision%29))
  ;[1 1 1] Camera (Ace)
  (Utilities|IsMenuClosed
    (:then
      (Pawn|Input|AddControllerYawInput (* AxisValue (Variables|Default|GetCamXSensitivity))))))

(event Input|KeyboardEvents|SpaceBar
  (params (Key :type Key%20Structure :default "None"))
  ;[1 1 1] Jump (Ace)
  (:Pressed
    (Utilities|IsMenuClosed
      (:then
        (Character|Jump)))))

(event Input|KeyboardEvents|K
  (params (Key :type Key%20Structure :default "None"))
  ;[1 1 1] Alternate between Gravity on and gravity off speed (gravity not included lol) (Ace)
  (:Pressed
    (Utilities|FlowControl|FlipFlop
      (:A
        (Variables|Default|SetMaxSpeed 0.2))
      (:B
        (Variables|Default|SetMaxSpeed 1.0)))))

(event Input|KeyboardEvents|2
  (params (Key :type Key%20Structure :default "None"))
  (bind _returnvalue (Game|GetPlayerController 0))
  (bind _returnvalue_2 (Game|GetPlayerController 0))
  ;[1 1 1] Ace WIP Sensitivity Slider widgets (you may ignore) (Ace)
  (:Pressed
    (Development|PrintString "Hello")
    (if (Game|IsGamePaused)
      (Game|SetGamePaused false)
      (Widget|RemovefromParent (stale _returnvalue_3))
      (Input|SetInputModeGameOnly _returnvalue_2 false)
      (Variables|/Script/Engine.PlayerController|SetbShowMouseCursor _returnvalue_2 false)
      (else
        (Game|SetGamePaused true)
        (bind _returnvalue_3 (UserInterface|CreateWidget "/Game/Coding/AceWest/BP_AceMenu.BP_AceMenu_C"))
        (UserInterface|Viewport|AddtoViewport _returnvalue_3 0)
        (Input|SetInputModeGameandUI _returnvalue 0 "DoNotLock" false false)
        (Variables|/Script/Engine.PlayerController|SetbShowMouseCursor _returnvalue true)))))

(fn ConstructionScript)