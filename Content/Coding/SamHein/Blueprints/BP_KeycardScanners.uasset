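; BP_KeycardScanners is an interactable keycard scanner that opens its referenced BP_Door once the player has obtained the keycard.
; On interaction it sets the scan-success animation sequence before checking KeyCardObtained in the BP_GameVariables game instance.
; If the keycard is held and the door is closed, a timeline slides both door halves apart along relative X and marks the door open.
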(event EventInteractwithObject
  (Class|SequenceEvaluatorLibrary|SetSequence (Variables|Default|GetIdScanSuccess) "/Game/Animations/RightID/IDScanSuccess_ANI_Anim.IDScanSuccess_ANI_Anim")
  (bind _asbp_door (Utilities|Casting|CastToBP_Door (Variables|Default|GetOtherActor)))
  ;[1 1 1] Check if Door Can be Opened
  (bind _asbp_game_variables (Utilities|Casting|CastToBP_GameVariables (Game|GetGameInstance)))
  (if (Variables|/Game/Coding/Luke_Samuelson/BP_GameVariables.BP_GameVariables_C|GetKeyCardObtained _asbp_game_variables)
    (if (not (Variables|/Game/Coding/Luke_Samuelson/Interactions/BP_Door.BP_Door_C|GetDoorOpen _asbp_door))
      (bind _newtrack_0 (Timeline|Timeline PlayFromStart)
        (:Update
          (Transformation|SetRelativeLocation (Variables|/Game/Coding/Luke_Samuelson/Interactions/BP_Door.BP_Door_C|GetDoorR _asbp_door) (Math|Vector|MakeVector (* _newtrack_0 1.9e+02) (.y (Variables|/Script/Engine.SceneComponent|GetRelativeLocation (Variables|/Game/Coding/Luke_Samuelson/Interactions/BP_Door.BP_Door_C|GetDoorR _asbp_door))) (.z (Variables|/Script/Engine.SceneComponent|GetRelativeLocation (Variables|/Game/Coding/Luke_Samuelson/Interactions/BP_Door.BP_Door_C|GetDoorR _asbp_door)))) false false)
          (Transformation|SetRelativeLocation (Variables|/Game/Coding/Luke_Samuelson/Interactions/BP_Door.BP_Door_C|GetDoorL _asbp_door) (Math|Vector|MakeVector (* _newtrack_0 -1.9e+02) (.y (Variables|/Script/Engine.SceneComponent|GetRelativeLocation (Variables|/Game/Coding/Luke_Samuelson/Interactions/BP_Door.BP_Door_C|GetDoorL _asbp_door))) (.z (Variables|/Script/Engine.SceneComponent|GetRelativeLocation (Variables|/Game/Coding/Luke_Samuelson/Interactions/BP_Door.BP_Door_C|GetDoorL _asbp_door)))) false false)
          (Variables|/Game/Coding/Luke_Samuelson/Interactions/BP_Door.BP_Door_C|SetDoorOpen _asbp_door true))))))

(fn ConstructionScript
  (|CallParentFunction))