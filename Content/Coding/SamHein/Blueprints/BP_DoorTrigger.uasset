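; BP_DoorTrigger is a trigger actor that slides a referenced BP_Door's two panels, apparently to close it, after something leaves its box.
; End overlap casts DoorActor to BP_Door, waits a fixed delay, then plays a timeline if DoorOpen is set.
; The timeline moves DoorR and DoorL in opposite directions along relative X and clears DoorOpen on each update.
; A failed cast only prints a message.
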(event OnComponentEndOverlap(Box)
  (params (OverlappedComponent :type Primitive%20Component%20Object%20Reference) (OtherActor :type Actor%20Object%20Reference) (OtherComp :type Primitive%20Component%20Object%20Reference) (OtherBodyIndex :type Integer))
  (bind _asbp_door (Utilities|Casting|CastToBP_Door (Variables|Default|GetDoorActor))
    (:then
      (Utilities|FlowControl|Delay 3.0)
      (if (Variables|/Game/Coding/Luke_Samuelson/Interactions/BP_Door.BP_Door_C|GetDoorOpen _asbp_door)
        (bind _newtrack_0 (Timeline|Timeline PlayFromStart)
          (:Update
            (Transformation|SetRelativeLocation (Variables|/Game/Coding/Luke_Samuelson/Interactions/BP_Door.BP_Door_C|GetDoorR _asbp_door) (Math|Vector|MakeVector (* _newtrack_0 1.9e+02) (.y (Variables|/Script/Engine.SceneComponent|GetRelativeLocation (Variables|/Game/Coding/Luke_Samuelson/Interactions/BP_Door.BP_Door_C|GetDoorR _asbp_door))) (.z (Variables|/Script/Engine.SceneComponent|GetRelativeLocation (Variables|/Game/Coding/Luke_Samuelson/Interactions/BP_Door.BP_Door_C|GetDoorR _asbp_door)))) false false)
            (Transformation|SetRelativeLocation (Variables|/Game/Coding/Luke_Samuelson/Interactions/BP_Door.BP_Door_C|GetDoorL _asbp_door) (Math|Vector|MakeVector (* _newtrack_0 -1.9e+02) (.y (Variables|/Script/Engine.SceneComponent|GetRelativeLocation (Variables|/Game/Coding/Luke_Samuelson/Interactions/BP_Door.BP_Door_C|GetDoorL _asbp_door))) (.z (Variables|/Script/Engine.SceneComponent|GetRelativeLocation (Variables|/Game/Coding/Luke_Samuelson/Interactions/BP_Door.BP_Door_C|GetDoorL _asbp_door)))) false false)
            (Variables|/Game/Coding/Luke_Samuelson/Interactions/BP_Door.BP_Door_C|SetDoorOpen _asbp_door false)))))
    (:CastFailed
      (Development|PrintString "Cast Failed"))))

(fn ConstructionScript)