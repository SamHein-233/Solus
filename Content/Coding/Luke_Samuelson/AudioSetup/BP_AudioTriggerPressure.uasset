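; BP_AudioTriggerPressure is a one-shot trigger actor that plays an assigned level sequence when the player character overlaps it.
; On overlap it starts the sequence and adds a W_Interaction widget to the viewport.
; After a one-second delay it removes all top-level W_Interaction widgets, not just the one it created, then destroys itself.
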(event Collision|EventActorBeginOverlap
  (params (OtherActor :type Actor%20Object%20Reference))
  (if (== OtherActor (Game|GetPlayerCharacter 0))
    (Sequencer|Player|Play (Variables|/Script/LevelSequence.LevelSequenceActor|GetSequencePlayer (Variables|Default|GetLevel%20Sequence%20to%20Play)) :!class /Script/MovieScene.MovieSceneSequencePlayer)
    (bind _returnvalue (UserInterface|CreateWidget "/Game/Coding/Luke_Samuelson/Widgets/W_Interaction.W_Interaction_C"))
    (UserInterface|Viewport|AddtoViewport _returnvalue 0)
    (Utilities|FlowControl|Delay 1.0)
    (bind _foundwidgets (Widget|GetAllWidgetsOfClass "/Game/Coding/Luke_Samuelson/Widgets/W_Interaction.W_Interaction_C" true))
    (Widget|RemovefromParent _foundwidgets)
    (Actor|DestroyActor)))

(fn ConstructionScript)