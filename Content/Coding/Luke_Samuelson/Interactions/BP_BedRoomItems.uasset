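; BP_BedRoomItems is a bedroom collectible that the player picks up through the InteractwithObject event.
; On interaction it destroys itself and increments BedroomObjectsCollected in the BP_GameVariables Game Instance.
; When the count equals three, it sets KeyCardObtained on the Game Instance and prints that flag for debugging.
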(event EventInteractwithObject
  ;[1 1 1] Pulling variables from Game Instance
  (bind _asbp_game_variables (Utilities|Casting|CastToBP_GameVariables (Game|GetGameInstance)))
  ;[1 1 1] Collecting Object
  (Actor|DestroyActor)
  (bind _result (Math|Integer|IncrementInt (Variables|/Game/Coding/Luke_Samuelson/BP_GameVariables.BP_GameVariables_C|GetBedroomObjectsCollected _asbp_game_variables))
    (:%20%20
      (bind _output_get (Variables|/Game/Coding/Luke_Samuelson/BP_GameVariables.BP_GameVariables_C|SetBedroomObjectsCollected _asbp_game_variables _result))
      (Math|Integer|CompareInt _output_get 3
        (:==
          (bind _output_get_2 (Variables|/Game/Coding/Luke_Samuelson/BP_GameVariables.BP_GameVariables_C|SetKeyCardObtained _asbp_game_variables true))
          (Development|PrintString (Utilities|String|ToString(Boolean) _output_get_2)))))))

(fn ConstructionScript
  (|CallParentFunction))