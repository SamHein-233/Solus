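; BP_AudioTrigger is an overlap trigger that plays an assigned level sequence when player character 0 enters it.
; After a Duration delay, it sets the IntroWalk flag on the BP_GameVariables game instance and adds a W_Interaction widget to the viewport.
; Any actor ending overlap removes top-level W_Interaction widgets, without checking that it is the player.
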(event Collision|EventActorBeginOverlap
  (params (OtherActor :type Actor%20Object%20Reference))
  (if (== OtherActor (Game|GetPlayerCharacter 0))
    (Sequencer|Player|Play (Variables|/Script/LevelSequence.LevelSequenceActor|GetSequencePlayer (Variables|Default|GetLevel%20Sequence%20to%20Play)) :!class /Script/MovieScene.MovieSceneSequencePlayer)
    (bind _asbp_game_variables (Utilities|Casting|CastToBP_GameVariables (Game|GetGameInstance))
      (:then
        (Utilities|FlowControl|Delay (Variables|Default|GetDuration))
        (Variables|/Game/Coding/Luke_Samuelson/BP_GameVariables.BP_GameVariables_C|SetIntro%20Walk _asbp_game_variables true)
        (Development|PrintString "Walk Set")
        (bind _returnvalue (UserInterface|CreateWidget "/Game/Coding/Luke_Samuelson/Widgets/W_Interaction.W_Interaction_C"))
        (UserInterface|Viewport|AddtoViewport _returnvalue 0))
      (:CastFailed
        (Development|PrintString "Cast Failed")))))

(event Collision|EventActorEndOverlap
  (params (OtherActor :type Actor%20Object%20Reference))
  (bind _foundwidgets (Widget|GetAllWidgetsOfClass "/Game/Coding/Luke_Samuelson/Widgets/W_Interaction.W_Interaction_C" true))
  (Widget|RemovefromParent _foundwidgets))

(fn ConstructionScript)