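; BP_GravCube is a cube actor whose gravity follows the Gravity variable on BP_PlayerCharacterACE.
; Every Tick it casts the player pawn to that character and copies the flag onto the Cube component.
; It then applies a fixed upward impulse and a random horizontal one, with each axis scaled by a random NegativeArray entry.
; These impulses fire every frame whatever the gravity state, provided the cast succeeds.
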(event EventTick
  (params (DeltaSeconds :type Float%20%28single-precision%29))
  (bind _returnvalue (Math|Random|RandomFloatinRange 5e+01 1e+02))
  (bind _negativearray (Variables|Default|GetnegativeArray))
  (bind _outitem (Utilities|Array|Random _negativearray))
  (bind _returnvalue_2 (* _returnvalue _outitem))
  (bind _asbp_player_character_ace (Utilities|Casting|CastToBP_PlayerCharacterACE (Game|Player|GetPlayerPawn 0)))
  (Physics|SetEnableGravity (Variables|Default|GetCube) (Variables|/Game/Coding/AceWest/BP_PlayerCharacterACE.BP_PlayerCharacterACE_C|Getgravity _asbp_player_character_ace))
  (Physics|AddImpulse (Variables|Default|GetCube) (Math|Vector|MakeVector 0.0 0.0 75.0) "None" false)
  (Physics|AddImpulse (Variables|Default|GetCube) (Math|Vector|MakeVector _returnvalue_2 _returnvalue_2 0.0) "None" false))

(fn ConstructionScript)