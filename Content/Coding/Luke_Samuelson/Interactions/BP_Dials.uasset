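; BP_Dials is an interactable circuit-puzzle dial that turns in 90-degree steps until the circuit is solved.
; Each interaction sets the mesh rotation, advances a four-state counter and writes it to the shared DialRotations array in BP_GameVariables at its DialCount index.
; A nested comparison chain checks 13 entries, skipping indices 2–4, then sets CircuitComplete.
; If the button and wire puzzles are also complete, it plays a Level Sequence.
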(event EventInteractwithObject
  (bind _returnvalue (Game|GetGameInstance))
  (bind _asbp_game_variables (Utilities|Casting|CastToBP_GameVariables _returnvalue))
  (if (not (Variables|/Game/Coding/Luke_Samuelson/BP_GameVariables.BP_GameVariables_C|GetCircuitComplete _asbp_game_variables))
    (Transformation|SetRelativeRotation (Variables|Default|GetDial) (Math|Rotator|MakeRotator 0.0 (* (Variables|Default|GetRotateCount) -9e+01) 0.0) false false)
    (bind _asbp_game_variables_2 (Utilities|Casting|CastToBP_GameVariables _returnvalue)
      (:then
        (bind _output_get (Variables|Default|SetRotateCount (Math|Integer|%(Integer) (+ (Variables|Default|GetRotateCount) 1) 4)))
        (Utilities|Array|SetArrayElem (Variables|/Game/Coding/Luke_Samuelson/BP_GameVariables.BP_GameVariables_C|GetDial%20Rotations _asbp_game_variables_2) (Variables|Default|GetDialCount) _output_get)
        (Math|Integer|CompareInt (Utilities|Array|Get(acopy) (Variables|/Game/Coding/Luke_Samuelson/BP_GameVariables.BP_GameVariables_C|GetDial%20Rotations _asbp_game_variables_2)) 1
          (:==
            (Math|Integer|CompareInt (Utilities|Array|Get(acopy) (Variables|/Game/Coding/Luke_Samuelson/BP_GameVariables.BP_GameVariables_C|GetDial%20Rotations _asbp_game_variables_2) 1) 3
              (:==
                (Math|Integer|CompareInt (Utilities|Array|Get(acopy) (Variables|/Game/Coding/Luke_Samuelson/BP_GameVariables.BP_GameVariables_C|GetDial%20Rotations _asbp_game_variables_2) 5) 2
                  (:==
                    (Math|Integer|CompareInt (Utilities|Array|Get(acopy) (Variables|/Game/Coding/Luke_Samuelson/BP_GameVariables.BP_GameVariables_C|GetDial%20Rotations _asbp_game_variables_2) 6) 3
                      (:==
                        (Math|Integer|CompareInt (Utilities|Array|Get(acopy) (Variables|/Game/Coding/Luke_Samuelson/BP_GameVariables.BP_GameVariables_C|GetDial%20Rotations _asbp_game_variables_2) 7) 3
                          (:==
                            (Math|Integer|CompareInt (Utilities|Array|Get(acopy) (Variables|/Game/Coding/Luke_Samuelson/BP_GameVariables.BP_GameVariables_C|GetDial%20Rotations _asbp_game_variables_2) 8) 2
                              (:==
                                (Math|Integer|CompareInt (Utilities|Array|Get(acopy) (Variables|/Game/Coding/Luke_Samuelson/BP_GameVariables.BP_GameVariables_C|GetDial%20Rotations _asbp_game_variables_2) 9) 3
                                  (:==
                                    (Math|Integer|CompareInt (Utilities|Array|Get(acopy) (Variables|/Game/Coding/Luke_Samuelson/BP_GameVariables.BP_GameVariables_C|GetDial%20Rotations _asbp_game_variables_2) 10) 2
                                      (:==
                                        (Math|Integer|CompareInt (Utilities|Array|Get(acopy) (Variables|/Game/Coding/Luke_Samuelson/BP_GameVariables.BP_GameVariables_C|GetDial%20Rotations _asbp_game_variables_2) 11) 3
                                          (:==
                                            (Math|Integer|CompareInt (Utilities|Array|Get(acopy) (Variables|/Game/Coding/Luke_Samuelson/BP_GameVariables.BP_GameVariables_C|GetDial%20Rotations _asbp_game_variables_2) 12) 1
                                              (:==
                                                (Math|Integer|CompareInt (Utilities|Array|Get(acopy) (Variables|/Game/Coding/Luke_Samuelson/BP_GameVariables.BP_GameVariables_C|GetDial%20Rotations _asbp_game_variables_2) 13) 1
                                                  (:==
                                                    (Math|Integer|CompareInt (Utilities|Array|Get(acopy) (Variables|/Game/Coding/Luke_Samuelson/BP_GameVariables.BP_GameVariables_C|GetDial%20Rotations _asbp_game_variables_2) 14)
                                                      (:==
                                                        (Math|Integer|CompareInt (Utilities|Array|Get(acopy) (Variables|/Game/Coding/Luke_Samuelson/BP_GameVariables.BP_GameVariables_C|GetDial%20Rotations _asbp_game_variables_2) 15) 1
                                                          (:==
                                                            (bind _asbp_game_variables_3 (Utilities|Casting|CastToBP_GameVariables (Game|GetGameInstance)))
                                                            (bind _output_get_2 (Variables|/Game/Coding/Luke_Samuelson/BP_GameVariables.BP_GameVariables_C|SetCircuitComplete _asbp_game_variables_3 true))
                                                            (Development|PrintString (Utilities|String|ToString(Boolean) _output_get_2))
                                                            (bind _asbp_game_variables_4 (Utilities|Casting|CastToBP_GameVariables (Game|GetGameInstance)))
                                                            (if (Math|Boolean|ANDBoolean (Variables|/Game/Coding/Luke_Samuelson/BP_GameVariables.BP_GameVariables_C|GetButtonsCompelte _asbp_game_variables_4) (Variables|/Game/Coding/Luke_Samuelson/BP_GameVariables.BP_GameVariables_C|GetCircuitComplete _asbp_game_variables_4) (Variables|/Game/Coding/Luke_Samuelson/BP_GameVariables.BP_GameVariables_C|GetWiresComplete _asbp_game_variables_4))
                                                              (Sequencer|Player|Play (Variables|/Script/LevelSequence.LevelSequenceActor|GetSequencePlayer (Variables|Default|GetLevel%20Sequencer)) :!class /Script/MovieScene.MovieSceneSequencePlayer)))))))))))))))))))))))))))))
      (:CastFailed
        (Development|PrintString "Cast Failed")))))

(fn ConstructionScript
  (|CallParentFunction))