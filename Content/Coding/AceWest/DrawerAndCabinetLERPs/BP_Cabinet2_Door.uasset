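; BP_Cabinet2_Door is an interactable cabinet door that swings open and closed.
; InteractwithObject toggles the Pulled flag, playing the PullOutDrawer timeline forward to open and reversing it to close.
; The timeline's update lerps the Cabinet2Door relative yaw from zero to the Distance variable, which serves as the swing angle despite its name.
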(event EventInteractwithObject
  (if (Variables|Default|GetPulled?)
    (Variables|Default|SetPulled? false)
    (bind _newtrack_0 (Timeline|Pull%20Out%20Drawer Reverse)
      (:Update
        (Transformation|SetRelativeRotation (Variables|Default|GetCabinet2_Door) (Math|Rotator|MakeRotator 0.0 0.0 (Math|Float|Lerp 0.0 (Variables|Default|GetDistance) _newtrack_0)) false false)))
    (else
      (Variables|Default|SetPulled? true)
      (Timeline|Pull%20Out%20Drawer Play))))

(fn ConstructionScript
  (|CallParentFunction))