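; BP_FinaleTrigger is an overlap trigger that runs the game's ending once all puzzles are solved.
; On overlap it reads the circuit, wires and buttons completion flags from the BP_GameVariables game instance.
; When all three are set, it plays a level sequence and disables the player character's WASD movement.
; After a fixed delay timed for the sequence, it clears all widgets and opens the credits level.
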(event Collision|EventActorBeginOverlap
  (params (OtherActor :type Actor%20Object%20Reference))
  (bind _asbp_game_variables (Utilities|Casting|CastToBP_GameVariables (Game|GetGameInstance))
    (:then
      (if (Math|Boolean|ANDBoolean (Variables|/Game/Coding/Luke_Samuelson/BP_GameVariables.BP_GameVariables_C|GetCircuitComplete _asbp_game_variables) (Variables|/Game/Coding/Luke_Samuelson/BP_GameVariables.BP_GameVariables_C|GetWiresComplete _asbp_game_variables) (Variables|/Game/Coding/Luke_Samuelson/BP_GameVariables.BP_GameVariables_C|GetButtonsCompelte _asbp_game_variables))
        (Sequencer|Player|Play (Variables|/Script/LevelSequence.LevelSequenceActor|GetSequencePlayer (Variables|Default|GetLevel%20Sequence%20to%20Play)) :!class /Script/MovieScene.MovieSceneSequencePlayer)
        (bind _asbp_player_character_ace (Utilities|Casting|CastToBP_PlayerCharacterACE (Game|GetPlayerCharacter 0)))
        (Variables|/Game/Coding/AceWest/BP_PlayerCharacterACE.BP_PlayerCharacterACE_C|SetWASD%20Movement _asbp_player_character_ace false)
        (Development|PrintString "AHHHHHH")
        (Utilities|FlowControl|Delay 6.3)
        (Viewport|RemoveAllWidgets)
        (Game|OpenLevel(byObjectReference) "/Game/Coding/Luke_Samuelson/Solus_Credits_Level.Solus_Credits_Level")))
    (:CastFailed
      (Development|PrintString "Cast Failed"))))

(fn ConstructionScript
  (|CallParentFunction))