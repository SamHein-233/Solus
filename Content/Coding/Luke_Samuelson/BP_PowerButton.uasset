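; BP_PowerButton is a button in an ordered power-button sequence puzzle, triggered by either an actor click or InteractwithObject.
; While the sequence is incomplete, it compares its ButtonValue to the expected entry in BP_GameVariables, the shared GameInstance holding the sequence and progress index.
; A match moves the Cylinder to a fixed pressed offset and advances the index, while a mismatch does nothing.
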(event EventInteractwithObject
  (bind _asbp_game_variables (Utilities|Casting|CastToBP_GameVariables (Game|GetGameInstance))
    (:then
      (if (not (Variables|/Game/Coding/Luke_Samuelson/BP_GameVariables.BP_GameVariables_C|GetButtonsCompelte _asbp_game_variables))
        (Math|Integer|CompareInt (Utilities|Array|Get(acopy) (Variables|/Game/Coding/Luke_Samuelson/BP_GameVariables.BP_GameVariables_C|GetPowerButtonValues _asbp_game_variables) (Variables|/Game/Coding/Luke_Samuelson/BP_GameVariables.BP_GameVariables_C|GetButtonsIndex _asbp_game_variables)) (Variables|Default|GetButtonValue)
          (:==
            (Transformation|SetRelativeLocation (Variables|Default|GetCylinder) "0.000000,-5.000000,0.000000" false false)
            (Math|Integer|IncrementInt (Variables|/Game/Coding/Luke_Samuelson/BP_GameVariables.BP_GameVariables_C|GetButtonsIndex _asbp_game_variables))))))
    (:CastFailed
      (Development|PrintString "Cast Failed"))))

(event MouseInput|EventActorOnClicked
  (params (ButtonPressed :type Key%20Structure :default "None"))
  (bind _asbp_game_variables (Utilities|Casting|CastToBP_GameVariables (Game|GetGameInstance))
    (:then
      (if (not (Variables|/Game/Coding/Luke_Samuelson/BP_GameVariables.BP_GameVariables_C|GetButtonsCompelte _asbp_game_variables))
        (Math|Integer|CompareInt (Utilities|Array|Get(acopy) (Variables|/Game/Coding/Luke_Samuelson/BP_GameVariables.BP_GameVariables_C|GetPowerButtonValues _asbp_game_variables) (Variables|/Game/Coding/Luke_Samuelson/BP_GameVariables.BP_GameVariables_C|GetButtonsIndex _asbp_game_variables)) (Variables|Default|GetButtonValue)
          (:==
            (Transformation|SetRelativeLocation (Variables|Default|GetCylinder) "0.000000,-5.000000,0.000000" false false)
            (Math|Integer|IncrementInt (Variables|/Game/Coding/Luke_Samuelson/BP_GameVariables.BP_GameVariables_C|GetButtonsIndex _asbp_game_variables))))))
    (:CastFailed
      (Development|PrintString "Cast Failed"))))

(fn ConstructionScript
  (|CallParentFunction))