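; Handle actor that pulls the player to itself when its goToHandle event is called.
; It disables player input, then plays a timeline that lerps the capsule's world location toward the handle mesh.
; Once within 100 units, it stops the timeline and re-enables input.
; Speed ramp events, axis-distance functions and a movement loop are leftover test code, with the loop left unconnected.
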(event Custom|goToHandle
  ;[1 1 1] Go to the handle
  (Input|DisableInput (Game|GetPlayerCharacter 0) 0)
  ;;[1 1 1] Start timeline for movement
  (bind _newtrack_0 (Timeline|updateHandleTimer PlayFromStart)
    (:Update
      (Variables|Default|Settime _newtrack_0)
      ;;[1 1 1] See if player is within 1m of the handle
      (Math|Float|CompareFloat (Math|Vector|Distance(Vector) (Transformation|GetWorldLocation (Variables|/Script/Engine.Character|GetCapsuleComponent (Game|GetPlayerCharacter 0))) (Transformation|GetWorldLocation (Variables|Default|GetSM_Handle))) 1e+02
        (:>
          ;;[1 1 1] Set the player world location
          (Transformation|SetWorldLocation (Variables|/Script/Engine.Character|GetCapsuleComponent (Game|GetPlayerCharacter 0)) (Math|Vector|Lerp(Vector) (Transformation|GetWorldLocation (Variables|/Script/Engine.Character|GetCapsuleComponent (Game|GetPlayerCharacter 0))) (Transformation|GetWorldLocation (Variables|Default|GetSM_Handle)) (Variables|Default|Gettime)) false false))
        (:==
          (Development|PrintString "finished moving" :!label _label)
          (Input|EnableInput (Game|GetPlayerCharacter 0) 0)
          (Timeline|updateHandleTimer Stop))
        (:<
          (goto _label))))))

(event Custom|playerSlowDown
  ;[1 1 1] Not used just for test purposes
  (Math|Float|CompareFloat (Variables|Default|Getspeed) 0.0
    (:>
      (Variables|Default|Setspeed (- (Variables|Default|Getspeed) 0.01)))
    (:==
      (Variables|Default|SetplayerSlowingDown false :!label _label))
    (:<
      (goto _label)))
  (CallFunction|UpdatePlayerLocation))

(event Custom|updatePlayerLocation
  ;[1 1 1] Not used just for test purposes
)

(event Custom|playerSpeedUp
  ;[1 1 1] Not used just for test purposes
  (Math|Float|CompareFloat (Variables|Default|Getspeed) 0.05
    (:>
      (Variables|Default|SetplayerSpeedingUp false :!label _label))
    (:==
      (goto _label))
    (:<
      (Variables|Default|Setspeed (+ (Variables|Default|Getspeed) 0.01))))
  (CallFunction|UpdatePlayerLocation))

(fn ConstructionScript)

(fn DistancetoHandle
  (bind _returnvalue (Game|GetPlayerCharacter 0))
  (bind _sm_handle (Variables|Default|GetSM_Handle))
  (bind _returnvalue_2 (Transformation|GetWorldLocation _sm_handle))
  (bind _capsulecomponent (Variables|/Script/Engine.Character|GetCapsuleComponent _returnvalue))
  (bind _returnvalue_3 (Transformation|GetWorldLocation _capsulecomponent))
  ;[1 1 1] Used in testing to get current distance from player to handle
  (Variables|Default|SetdistanceToHandleX (- (.x _returnvalue_3) (.x _returnvalue_2)))
  (Variables|Default|SetdistanceToHandleY (- (.y _returnvalue_3) (.y _returnvalue_2)))
  (Variables|Default|SetdistanceToHandleZ (- (.z _returnvalue_3) (.z _returnvalue_2))))

(fn StartDistancetoHandle
  (bind _returnvalue (Game|GetPlayerCharacter 0))
  (bind _sm_handle (Variables|Default|GetSM_Handle))
  (bind _returnvalue_2 (Transformation|GetWorldLocation _sm_handle))
  (bind _capsulecomponent (Variables|/Script/Engine.Character|GetCapsuleComponent _returnvalue))
  (bind _returnvalue_3 (Transformation|GetWorldLocation _capsulecomponent))
  ;[1 1 1] Used in testing to get starting distance from player to handle
  (Variables|Default|SetstartDistanceToHandleX (- (.x _returnvalue_3) (.x _returnvalue_2)))
  (Variables|Default|SetstartDistanceToHandleY (- (.y _returnvalue_3) (.y _returnvalue_2)))
  (Variables|Default|SetstartDistanceToHandleZ (- (.z _returnvalue_3) (.z _returnvalue_2))))