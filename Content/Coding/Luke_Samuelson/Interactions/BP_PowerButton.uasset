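; BP_PowerButton is one button in an ordered-press power puzzle, triggered by clicking or interacting.
; It compares its value to the next expected one in BP_GameVariables; a match depresses it, turns it green and advances the shared index, while a mismatch only plays a decline sound.
; The fifth match completes the puzzle and restores walking.
; If circuit and wire puzzles are also complete, it plays a level sequence with WASD movement temporarily disabled.
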(event EventInteractwithObject
  (bind _asbp_game_variables (Utilities|Casting|CastToBP_GameVariables (Game|GetGameInstance))
    (:then
      (if (not (Variables|/Game/Coding/Luke_Samuelson/BP_GameVariables.BP_GameVariables_C|GetButtonsCompelte _asbp_game_variables))
        (Math|Integer|CompareInt (Utilities|Array|Get(acopy) (Variables|/Game/Coding/Luke_Samuelson/BP_GameVariables.BP_GameVariables_C|GetPowerButtonValues _asbp_game_variables) (Variables|/Game/Coding/Luke_Samuelson/BP_GameVariables.BP_GameVariables_C|GetButtonsIndex _asbp_game_variables)) (Variables|Default|GetButtonValue)
          (:>
            (Audio|PlaySound2D "/Game/Audio/Ambient/Sounds/Decline_Harmony.Decline_Harmony" 1.0 1.0 0.0 0 0 :!label _label))
          (:==
            (Audio|PlaySound2D "/Game/Audio/Ambient/Sounds/Accepting_Harmony.Accepting_Harmony" 1.0 1.0 0.0 0 0)
            (Transformation|SetRelativeLocation (Variables|Default|GetButton) "0.000000,-5.000000,0.000000" false false)
            (Rendering|Material|SetMaterial (Variables|Default|GetButton) 0 "/Game/Coding/Luke_Samuelson/Materials/MI_EmissiveGreen.MI_EmissiveGreen")
            (bind _result (Math|Integer|IncrementInt (Variables|/Game/Coding/Luke_Samuelson/BP_GameVariables.BP_GameVariables_C|GetButtonsIndex _asbp_game_variables))
              (:%20%20
                (Math|Integer|CompareInt _result 5
                  (:==
                    (bind _asbp_game_variables_2 (Utilities|Casting|CastToBP_GameVariables (Game|GetGameInstance)))
                    (Variables|/Game/Coding/Luke_Samuelson/BP_GameVariables.BP_GameVariables_C|SetButtonsCompelte _asbp_game_variables_2 true)
                    (Development|PrintString "Buttons Complete")
                    (Pawn|Components|CharacterMovement|SetMovementMode (Variables|/Script/Engine.Character|GetCharacterMovement (Game|GetPlayerCharacter 0)) "MOVE_Walking" 0)
                    (bind _asbp_game_variables_3 (Utilities|Casting|CastToBP_GameVariables (Game|GetGameInstance)))
                    (if (Math|Boolean|ANDBoolean (Variables|/Game/Coding/Luke_Samuelson/BP_GameVariables.BP_GameVariables_C|GetButtonsCompelte _asbp_game_variables_3) (Variables|/Game/Coding/Luke_Samuelson/BP_GameVariables.BP_GameVariables_C|GetCircuitComplete _asbp_game_variables_3) (Variables|/Game/Coding/Luke_Samuelson/BP_GameVariables.BP_GameVariables_C|GetWiresComplete _asbp_game_variables_3))
                      (bind _asbp_player_character_ace (Utilities|Casting|CastToBP_PlayerCharacterACE (Game|GetPlayerCharacter 0)))
                      (Variables|/Game/Coding/AceWest/BP_PlayerCharacterACE.BP_PlayerCharacterACE_C|SetWASD%20Movement _asbp_player_character_ace false)
                      (Sequencer|Player|Play (Variables|/Script/LevelSequence.LevelSequenceActor|GetSequencePlayer (Variables|Default|GetLevel%20Sequencer)) :!class /Script/MovieScene.MovieSceneSequencePlayer)
                      (Utilities|FlowControl|Delay 13.5)
                      (Variables|/Game/Coding/AceWest/BP_PlayerCharacterACE.BP_PlayerCharacterACE_C|SetWASD%20Movement _asbp_player_character_ace true)))))))
          (:<
            (goto _label)))))
    (:CastFailed
      (Development|PrintString "Cast Failed"))))

(event MouseInput|EventActorOnClicked
  (params (ButtonPressed :type Key%20Structure :default "None"))
  (bind _asbp_game_variables (Utilities|Casting|CastToBP_GameVariables (Game|GetGameInstance))
    (:then
      (if (not (Variables|/Game/Coding/Luke_Samuelson/BP_GameVariables.BP_GameVariables_C|GetButtonsCompelte _asbp_game_variables))
        (Math|Integer|CompareInt (Utilities|Array|Get(acopy) (Variables|/Game/Coding/Luke_Samuelson/BP_GameVariables.BP_GameVariables_C|GetPowerButtonValues _asbp_game_variables) (Variables|/Game/Coding/Luke_Samuelson/BP_GameVariables.BP_GameVariables_C|GetButtonsIndex _asbp_game_variables)) (Variables|Default|GetButtonValue)
          (:>
            (Audio|PlaySound2D "/Game/Audio/Ambient/Sounds/Decline_Harmony.Decline_Harmony" 1.0 1.0 0.0 0 0 :!label _label))
          (:==
            (Audio|PlaySound2D "/Game/Audio/Ambient/Sounds/Accepting_Harmony.Accepting_Harmony" 1.0 1.0 0.0 0 0)
            (Transformation|SetRelativeLocation (Variables|Default|GetButton) "0.000000,-5.000000,0.000000" false false)
            (Rendering|Material|SetMaterial (Variables|Default|GetButton) 0 "/Game/Coding/Luke_Samuelson/Materials/MI_EmissiveGreen.MI_EmissiveGreen")
            (bind _result (Math|Integer|IncrementInt (Variables|/Game/Coding/Luke_Samuelson/BP_GameVariables.BP_GameVariables_C|GetButtonsIndex _asbp_game_variables))
              (:%20%20
                (Math|Integer|CompareInt _result 5
                  (:==
                    (bind _asbp_game_variables_2 (Utilities|Casting|CastToBP_GameVariables (Game|GetGameInstance)))
                    (Variables|/Game/Coding/Luke_Samuelson/BP_GameVariables.BP_GameVariables_C|SetButtonsCompelte _asbp_game_variables_2 true)
                    (Development|PrintString "Buttons Complete")
                    (Pawn|Components|CharacterMovement|SetMovementMode (Variables|/Script/Engine.Character|GetCharacterMovement (Game|GetPlayerCharacter 0)) "MOVE_Walking" 0)
                    (bind _asbp_game_variables_3 (Utilities|Casting|CastToBP_GameVariables (Game|GetGameInstance)))
                    (if (Math|Boolean|ANDBoolean (Variables|/Game/Coding/Luke_Samuelson/BP_GameVariables.BP_GameVariables_C|GetButtonsCompelte _asbp_game_variables_3) (Variables|/Game/Coding/Luke_Samuelson/BP_GameVariables.BP_GameVariables_C|GetCircuitComplete _asbp_game_variables_3) (Variables|/Game/Coding/Luke_Samuelson/BP_GameVariables.BP_GameVariables_C|GetWiresComplete _asbp_game_variables_3))
                      (bind _asbp_player_character_ace (Utilities|Casting|CastToBP_PlayerCharacterACE (Game|GetPlayerCharacter 0)))
                      (Variables|/Game/Coding/AceWest/BP_PlayerCharacterACE.BP_PlayerCharacterACE_C|SetWASD%20Movement _asbp_player_character_ace false)
                      (Sequencer|Player|Play (Variables|/Script/LevelSequence.LevelSequenceActor|GetSequencePlayer (Variables|Default|GetLevel%20Sequencer)) :!class /Script/MovieScene.MovieSceneSequencePlayer)
                      (Utilities|FlowControl|Delay 13.5)
                      (Variables|/Game/Coding/AceWest/BP_PlayerCharacterACE.BP_PlayerCharacterACE_C|SetWASD%20Movement _asbp_player_character_ace true)))))))
          (:<
            (goto _label)))))
    (:CastFailed
      (Development|PrintString "Cast Failed"))))

(fn ConstructionScript
  (|CallParentFunction))