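; First-person-style player character handling movement, jump, camera look with sensitivity and Y-invert, and a K toggle for slower forward/back movement.
; Each tick a camera line trace stores the looked-at actor, which Interact triggers if it is a BP_MasterInteract.
; BeginPlay restores or creates the "save1" position save; T reloads it, while savepoint overlap saves to an empty slot name.
; Key 1 toggles pause and the WIP BP_AceMenu widget.
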(event EventTick
  (params (DeltaSeconds :type Float%20%28single-precision%29))
  (bind _returnvalue (Game|GetPlayerCameraManager 0))
  (bind _returnvalue_2 (Transformation|GetActorLocation _returnvalue))
  ;[1 1 1] Interact (Luke)
  (bind (_outhit _returnvalue_3) (Collision|LineTraceByChannel _returnvalue_2 (+ (* (Transformation|GetActorForwardVector _returnvalue) (Variables|Default|GetDistance%20Forward%20Look)) _returnvalue_2) "TraceTypeQuery1" false 0 "None"))
  (if _returnvalue_3
    (Variables|Default|SetObjLookedAt (.HitActor (Collision|BreakHitResult _outhit)))
    (else
      (Variables|Default|SetObjLookedAt 0))))

(event Collision|EventActorBeginOverlap
  (params (OtherActor :type Actor%20Object%20Reference))
  (bind _as_bp_save_game (Variables|Default|GetAs%20BP%20Save%20Game))
  (if (== "/Game/Coding/Luke_Samuelson/SaveSystem/BP_Savepoint.BP_Savepoint" OtherActor)
    (bind _returnvalue (SaveGame|DoesSaveGameExist "save1"))
    (if _returnvalue
      (Variables|/Game/Coding/Luke_Samuelson/SaveSystem/BP_SaveGame.BP_SaveGame_C|SetPlayerPos _as_bp_save_game (Transformation|GetActorTransform))
      (SaveGame|SaveGametoSlot _as_bp_save_game)
      (Development|PrintString "Game Saved"))))

(event EventBeginPlay
  ;[1 1 1] CamYInvert (Ace)
  (if (Variables|Default|GetCamYInvert)
    (Variables|Default|SetCamYInvertVal -1)
    (else
      (Variables|Default|SetCamYInvertVal 1)))
  (bind _returnvalue (SaveGame|DoesSaveGameExist "save1"))
  (if _returnvalue
    (bind _returnvalue_2 (SaveGame|LoadGamefromSlot "save1"))
    (bind _asbp_save_game (Utilities|Casting|CastToBP_SaveGame _returnvalue_2))
    (Variables|Default|SetAs%20BP%20Save%20Game _asbp_save_game)
    (Transformation|SetActorTransform (Variables|/Game/Coding/Luke_Samuelson/SaveSystem/BP_SaveGame.BP_SaveGame_C|GetPlayerPos _asbp_save_game))
    (else
      (bind _returnvalue_3 (SaveGame|CreateSaveGameObject "/Game/Coding/Luke_Samuelson/SaveSystem/BP_SaveGame.BP_SaveGame_C"))
      (Variables|/Game/Coding/Luke_Samuelson/SaveSystem/BP_SaveGame.BP_SaveGame_C|SetPlayerPos _returnvalue_3 (Transformation|GetActorTransform))
      (SaveGame|SaveGametoSlot _returnvalue_3 "save1")
      (Variables|Default|SetAs%20BP%20Save%20Game _returnvalue_3))))

(event Input|ActionEvents|InputActionInteract
  (params (Key :type Key%20Structure))
  ;[1 1 1] Interact (Luke)
  (:Pressed
    (bind _asbp_master_interact (Utilities|Casting|CastToBP_MasterInteract (Variables|Default|GetObjLookedAt)))
    (Default|InteractwithObject _asbp_master_interact)))

(event Input|AxisEvents|InputAxisForwardBack
  (params (AxisValue :type Float%20%28single-precision%29))
  ;[1 1 1] WASD Movement (Ace)
  (Pawn|Input|AddMovementInput (Transformation|GetActorForwardVector) (* (Variables|Default|GetMaxSpeed) AxisValue) false))

(event Input|AxisEvents|InputAxisLeftRight
  (params (AxisValue :type Float%20%28single-precision%29))
  ;[1 1 1] WASD Movement (Ace)
  (Pawn|Input|AddMovementInput (Transformation|GetActorRightVector) AxisValue false))

(event Input|AxisEvents|InputAxisCameraY
  (params (AxisValue :type Float%20%28single-precision%29))
  ;[1 1 1] Camera (Ace)
  (Pawn|Input|AddControllerPitchInput (* AxisValue (Variables|Default|GetCamYInvertVal) (Variables|Default|GetCamYSensitivity))))

(event Input|AxisEvents|InputAxisCameraX
  (params (AxisValue :type Float%20%28single-precision%29))
  ;[1 1 1] Camera (Ace)
  (Pawn|Input|AddControllerYawInput (* AxisValue (Variables|Default|GetCamXSensitivity))))

(event Input|KeyboardEvents|SpaceBar
  (params (Key :type Key%20Structure))
  ;[1 1 1] Jump (Ace)
  (:Pressed
    (Character|Jump)))

(event Input|KeyboardEvents|K
  (params (Key :type Key%20Structure))
  ;[1 1 1] Alternate between Gravity on and gravity off speed (gravity not included lol) (Ace)
  (:Pressed
    (Utilities|FlowControl|FlipFlop
      (:A
        (Variables|Default|SetMaxSpeed 0.2))
      (:B
        (Variables|Default|SetMaxSpeed 1.0)))))

(event Input|KeyboardEvents|1
  (params (Key :type Key%20Structure))
  (bind _returnvalue (Game|GetPlayerController 0))
  (bind _returnvalue_2 (Game|GetPlayerController 0))
  ;[1 1 1] Ace WIP Sensitivity Slider widgets (you may ignore) (Ace)
  (:Pressed
    (Development|PrintString "Hello")
    (if (Game|IsGamePaused)
      (Game|SetGamePaused false)
      (Widget|RemovefromParent (stale _returnvalue_3))
      (Input|SetInputModeGameOnly _returnvalue false)
      (Variables|/Script/Engine.PlayerController|SetbShowMouseCursor _returnvalue false)
      (else
        (Game|SetGamePaused true)
        (bind _returnvalue_3 (UserInterface|CreateWidget "/Game/Coding/AceWest/BP_AceMenu.BP_AceMenu_C"))
        (UserInterface|Viewport|AddtoViewport _returnvalue_3 0)
        (Input|SetInputModeGameandUI _returnvalue_2 0 "DoNotLock" false false)
        (Variables|/Script/Engine.PlayerController|SetbShowMouseCursor _returnvalue_2 true)))))

(event Input|KeyboardEvents|T
  (params (Key :type Key%20Structure))
  (:Pressed
    (bind _returnvalue (SaveGame|DoesSaveGameExist "save1"))
    (if _returnvalue
      (Transformation|SetActorTransform (Variables|/Game/Coding/Luke_Samuelson/SaveSystem/BP_SaveGame.BP_SaveGame_C|GetPlayerPos (Variables|Default|GetAs%20BP%20Save%20Game)))
      (Development|PrintString "Game Loaded"))))

(fn ConstructionScript)