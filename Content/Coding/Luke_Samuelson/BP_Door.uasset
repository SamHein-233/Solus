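; BP_Door is a keycard-gated sliding door that opens on interaction if the game instance BP_GameVariables has KeyCardObtained set.
; Two timelines slide the Door along world X, adding a scaled offset to its current location each update, and toggle DoorOpen.
; When a Character leaves the Sphere, an open door slides back; otherwise a W_NoAccess widget appears for a few seconds before all widgets are removed.
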(event OnComponentEndOverlap(Sphere)
  (params (OverlappedComponent :type Primitive%20Component%20Object%20Reference) (OtherActor :type Actor%20Object%20Reference) (OtherComp :type Primitive%20Component%20Object%20Reference) (OtherBodyIndex :type Integer))
  (bind _door (Variables|Default|GetDoor))
  (bind _returnvalue (Transformation|GetWorldLocation _door))
  (Utilities|Casting|CastToCharacter OtherActor)
  (if (Variables|Default|GetDoorOpen)
    (bind _newtrack_0 (Timeline|Timeline_0 PlayFromStart)
      (:Update
        (Transformation|SetWorldLocation (Variables|Default|GetDoor) (Math|Vector|MakeVector (+ (.x _returnvalue) (* _newtrack_0 -1.9)) (.y _returnvalue) (.z _returnvalue)) false false)
        (Variables|Default|SetDoorOpen false)))
    (else
      (bind _returnvalue_2 (UserInterface|CreateWidget "/Game/Coding/SamHein/Widgets/W_NoAccess.W_NoAccess_C"))
      (bind _output_get (Variables|Default|SetNewVar _returnvalue_2))
      (UserInterface|Viewport|AddtoViewport _output_get 0)
      (Utilities|FlowControl|Delay 3.0)
      (Viewport|RemoveAllWidgets))))

(event EventInteractwithObject
  (bind _door (Variables|Default|GetDoor))
  (bind _returnvalue (Transformation|GetWorldLocation _door))
  (bind _asbp_game_variables (Utilities|Casting|CastToBP_GameVariables (Game|GetGameInstance)))
  (if (and (Variables|/Game/Coding/Luke_Samuelson/BP_GameVariables.BP_GameVariables_C|GetKeyCardObtained _asbp_game_variables) (not (Variables|Default|GetDoorOpen)))
    (bind _newtrack_0 (Timeline|Timeline PlayFromStart)
      (:Update
        (Transformation|SetWorldLocation (Variables|Default|GetDoor) (Math|Vector|MakeVector (+ (* _newtrack_0 1.9) (.x _returnvalue)) (.y _returnvalue) (.z _returnvalue)) false false)
        (Variables|Default|SetDoorOpen true)))))

(fn ConstructionScript
  (|CallParentFunction))