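; BP_WireStart is an interactable start node in a wire-matching puzzle, active until the wires are complete.
; Interacting stores its WireCount in the BP_GameVariables game instance and, if that equals the stored end wire, marks it complete and swaps materials on both ends.
; When every wire through index four is done, it restores walking.
; If buttons and circuit are also complete, it fades music and plays a sequence, pausing WASD movement.
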(event EventInteractwithObject
  (bind _wire_count (Variables|Default|GetWire%20Count))
  ;[1 1 1] Check to See if Completed
  (bind _asbp_game_variables (Utilities|Casting|CastToBP_GameVariables (Game|GetGameInstance)))
  (if (not (Variables|/Game/Coding/Luke_Samuelson/BP_GameVariables.BP_GameVariables_C|GetWiresComplete _asbp_game_variables))
    (Development|PrintString "Pressed")
    ;[1 1 1] Pull Needed Variables
    (bind _asbp_game_variables_2 (Utilities|Casting|CastToBP_GameVariables (Game|GetGameInstance))
      (:then
        (bind _output_get (Variables|/Game/Coding/Luke_Samuelson/BP_GameVariables.BP_GameVariables_C|SetTempStartWire _asbp_game_variables_2 _wire_count))
        ;[1 1 1] Set Instance to Complete
        (Math|Integer|CompareInt _output_get (Variables|/Game/Coding/Luke_Samuelson/BP_GameVariables.BP_GameVariables_C|GetTempEndWire _asbp_game_variables_2)
          (:==
            (Utilities|Array|SetArrayElem (Variables|/Game/Coding/Luke_Samuelson/BP_GameVariables.BP_GameVariables_C|GetWireComplete _asbp_game_variables_2) _wire_count true)
            ;[1 1 1] Turn Off Flash
            (bind _array_index (Utilities|Array|ForEachLoopwithBreak (Variables|/Game/Coding/Luke_Samuelson/BP_GameVariables.BP_GameVariables_C|GetWireComplete _asbp_game_variables_2))
              (:LoopBody
                (Rendering|Material|SetMaterial (Variables|Default|GetWireStartCube) _array_index (Variables|Default|GetMaterialChange))
                (bind _asbp_wire_end (Utilities|Casting|CastToBP_WireEnd (Variables|Default|GetMatchingEnd)))
                (Rendering|Material|SetMaterial (Variables|/Game/Coding/Luke_Samuelson/Interactions/BP_WireEnd.BP_WireEnd_C|GetWireEndCube _asbp_wire_end) _array_index (Variables|/Game/Coding/Luke_Samuelson/Interactions/BP_WireEnd.BP_WireEnd_C|GetMaterialChange _asbp_wire_end)))
              (:Completed
                ;[1 1 1] Check Complete
                (bind _asbp_game_variables_3 (Utilities|Casting|CastToBP_GameVariables (Game|GetGameInstance)))
                (bind (_array_element _array_index_2) (Utilities|Array|ForEachLoopwithBreak (Variables|/Game/Coding/Luke_Samuelson/BP_GameVariables.BP_GameVariables_C|GetWireComplete _asbp_game_variables_3) :!label _label)
                  (:LoopBody
                    (if _array_element
                      (Math|Integer|CompareInt _array_index_2 4
                        (:==
                          (Audio|PlaySound2D "/Game/Audio/Ambient/Sounds/Accepting_Harmony.Accepting_Harmony" 1.0 1.0 0.0 0 0)
                          (Variables|/Game/Coding/Luke_Samuelson/BP_GameVariables.BP_GameVariables_C|SetWiresComplete _asbp_game_variables_3 true)
                          (Development|PrintString "Wires Compelte")
                          (Pawn|Components|CharacterMovement|SetMovementMode (Variables|/Script/Engine.Character|GetCharacterMovement (Game|GetPlayerCharacter 0)) "MOVE_Walking" 0)
                          (bind _asbp_game_variables_4 (Utilities|Casting|CastToBP_GameVariables (Game|GetGameInstance)))
                          (if (Math|Boolean|ANDBoolean (Variables|/Game/Coding/Luke_Samuelson/BP_GameVariables.BP_GameVariables_C|GetButtonsCompelte _asbp_game_variables_4) (Variables|/Game/Coding/Luke_Samuelson/BP_GameVariables.BP_GameVariables_C|GetCircuitComplete _asbp_game_variables_4) (Variables|/Game/Coding/Luke_Samuelson/BP_GameVariables.BP_GameVariables_C|GetWiresComplete _asbp_game_variables_4))
                            (bind _asbp_screen_changer (Utilities|Casting|CastToBP_ScreenChanger (Variables|Default|GetScreen%20Changer)))
                            (Audio|Components|Audio|FadeOut (Variables|/Game/Coding/SamHein/Blueprints/BP_ScreenChanger.BP_ScreenChanger_C|GetMusicRef _asbp_screen_changer) 0.0 0.0 "Linear" :!class /Script/Engine.AudioComponent)
                            (bind _asbp_player_character_ace (Utilities|Casting|CastToBP_PlayerCharacterACE (Game|GetPlayerCharacter 0)))
                            (Variables|/Game/Coding/AceWest/BP_PlayerCharacterACE.BP_PlayerCharacterACE_C|SetWASD%20Movement _asbp_player_character_ace false)
                            (Sequencer|Player|Play (Variables|/Script/LevelSequence.LevelSequenceActor|GetSequencePlayer (Variables|Default|GetLevel%20Sequencer)) :!class /Script/MovieScene.MovieSceneSequencePlayer)
                            (Utilities|FlowControl|Delay 13.5)
                            (Variables|/Game/Coding/AceWest/BP_PlayerCharacterACE.BP_PlayerCharacterACE_C|SetWASD%20Movement _asbp_player_character_ace true))))
                      (else
                        (goto _label Break))))))))))
      (:CastFailed
        (Development|PrintString "Button Cast Failed")))))

(fn ConstructionScript
  (|CallParentFunction))