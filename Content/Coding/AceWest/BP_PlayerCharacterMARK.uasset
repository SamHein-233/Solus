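; Player character with axis movement, jump, adjustable camera look, and visibility signalling for disappearing items.
; K toggles a reduced forward/back speed, and key 1 pauses and shows the work-in-progress BP_AceMenu.
; FOV component overlaps set each BP_DisappearingItem's looked-at and visibility flags, while capsule overlaps set its in-room flag.
; An unfinished line-trace alternative and a pause-test loop are left disconnected.
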(event OnComponentBeginOverlap(FOV)
  (params (OverlappedComponent :type Primitive%20Component%20Object%20Reference) (OtherActor :type Actor%20Object%20Reference) (OtherComp :type Primitive%20Component%20Object%20Reference) (OtherBodyIndex :type Integer) (bFromSweep :type Boolean) (SweepResult :type Hit%20Result%20Structure%20%28by%20ref%29))
  ;[0.2753 1 0.5184] Component Overlap BP_DissappearingItem w/ FOV (MARK)
  (bind _asbp_disappearing_item (Utilities|Casting|CastToBP_DisappearingItem OtherActor))
  (Variables|/Game/Coding/BP_DisappearingItem.BP_DisappearingItem_C|SetIsNotVisible _asbp_disappearing_item false)
  (Variables|/Game/Coding/BP_DisappearingItem.BP_DisappearingItem_C|SetLookedAt _asbp_disappearing_item true))

(event OnComponentEndOverlap(FOV)
  (params (OverlappedComponent :type Primitive%20Component%20Object%20Reference) (OtherActor :type Actor%20Object%20Reference) (OtherComp :type Primitive%20Component%20Object%20Reference) (OtherBodyIndex :type Integer))
  ;[0.2753 1 0.5184] Component Overlap BP_DissappearingItem w/ FOV (MARK)
  (bind _asbp_disappearing_item (Utilities|Casting|CastToBP_DisappearingItem OtherActor))
  (Variables|/Game/Coding/BP_DisappearingItem.BP_DisappearingItem_C|SetIsNotVisible _asbp_disappearing_item true))

(event OnComponentBeginOverlap(CapsuleComponent)
  (params (OverlappedComponent :type Primitive%20Component%20Object%20Reference) (OtherActor :type Actor%20Object%20Reference) (OtherComp :type Primitive%20Component%20Object%20Reference) (OtherBodyIndex :type Integer) (bFromSweep :type Boolean) (SweepResult :type Hit%20Result%20Structure%20%28by%20ref%29))
  ;[0.2753 1 0.5184] Component Overlap BP_DissappearingItem w/ FOV (MARK)
  (bind _asbp_disappearing_item (Utilities|Casting|CastToBP_DisappearingItem OtherActor))
  (Variables|/Game/Coding/BP_DisappearingItem.BP_DisappearingItem_C|SetInTheRoom _asbp_disappearing_item true))

(event OnComponentEndOverlap(CapsuleComponent)
  (params (OverlappedComponent :type Primitive%20Component%20Object%20Reference) (OtherActor :type Actor%20Object%20Reference) (OtherComp :type Primitive%20Component%20Object%20Reference) (OtherBodyIndex :type Integer))
  ;[0.2753 1 0.5184] Component Overlap BP_DissappearingItem w/ FOV (MARK)
  (bind _asbp_disappearing_item (Utilities|Casting|CastToBP_DisappearingItem OtherActor))
  (Variables|/Game/Coding/BP_DisappearingItem.BP_DisappearingItem_C|SetInTheRoom _asbp_disappearing_item false))

(event EventBeginPlay
  ;[1 1 1] CamYInvert (Ace)
  (if (Variables|Default|GetCamYInvert)
    (Variables|Default|SetCamYInvertVal -1)
    (else
      (Variables|Default|SetCamYInvertVal 1))))

(event Input|AxisEvents|InputAxisForwardBack
  (params (AxisValue :type Float%20%28single-precision%29))
  ;[1 1 1] WASD Movement (Ace)
  (Pawn|Input|AddMovementInput (Transformation|GetActorForwardVector) (* (Variables|Default|GetMaxSpeed) AxisValue) false))

(event Input|AxisEvents|InputAxisLeftRight
  (params (AxisValue :type Float%20%28single-precision%29))
  ;[1 1 1] WASD Movement (Ace)
  (Pawn|Input|AddMovementInput (Transformation|GetActorRightVector) AxisValue false))

(event Input|AxisEvents|InputAxisCameraY
  (params (AxisValue :type Float%20%28single-precision%29))
  ;[1 1 1] Camera (Ace)
  (Pawn|Input|AddControllerPitchInput (* AxisValue (Variables|Default|GetCamYInvertVal) (Variables|Default|GetCamYSensitivity))))

(event Input|AxisEvents|InputAxisCameraX
  (params (AxisValue :type Float%20%28single-precision%29))
  ;[1 1 1] Camera (Ace)
  (Pawn|Input|AddControllerYawInput (* AxisValue (Variables|Default|GetCamXSensitivity))))

(event Input|KeyboardEvents|SpaceBar
  (params (Key :type Key%20Structure :default "None"))
  ;[1 1 1] Jump (Ace)
  (:Pressed
    (Character|Jump)))

(event Input|KeyboardEvents|K
  (params (Key :type Key%20Structure :default "None"))
  ;[1 1 1] Alternate between Gravity on and gravity off speed (gravity not included lol) (Ace)
  (:Pressed
    (Utilities|FlowControl|FlipFlop
      (:A
        (Variables|Default|SetMaxSpeed 0.2))
      (:B
        (Variables|Default|SetMaxSpeed 1.0)))))

(event Input|KeyboardEvents|1
  (params (Key :type Key%20Structure :default "None"))
  (bind _returnvalue (Game|GetPlayerController 0))
  (bind _returnvalue_2 (Game|GetPlayerController 0))
  ;[1 1 1] Ace WIP Sensitivity Slider widgets (you may ignore) (Ace)
  (:Pressed
    (Development|PrintString "Hello")
    (if (Game|IsGamePaused)
      (Game|SetGamePaused false)
      (Widget|RemovefromParent (stale _returnvalue_3))
      (Input|SetInputModeGameOnly _returnvalue false)
      (Variables|/Script/Engine.PlayerController|SetbShowMouseCursor _returnvalue false)
      (else
        (Game|SetGamePaused true)
        (bind _returnvalue_3 (UserInterface|CreateWidget "/Game/Coding/AceWest/BP_AceMenu.BP_AceMenu_C"))
        (UserInterface|Viewport|AddtoViewport _returnvalue_3 0)
        (Input|SetInputModeGameandUI _returnvalue_2 0 "DoNotLock" false false)
        (Variables|/Script/Engine.PlayerController|SetbShowMouseCursor _returnvalue_2 true)))))

(fn ConstructionScript)