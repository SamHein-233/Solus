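; First-person player character with WASD movement, mouse look, jump, crouch, inventory helpers and savepoint saving.
; Input events drive pausing and a delayed, tabbed menu for map and settings, using widgets built in CreateCrosshair.
; Tick traces for interactables and simulates zero gravity with alternating upward forces, slamming down after generator-room float.
; FOV and capsule overlaps update disappearing items' visibility and room flags, while a separate trace on E targets handles.
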(event OnComponentBeginOverlap(FOV)
  (params (OverlappedComponent :type Primitive%20Component%20Object%20Reference) (OtherActor :type Actor%20Object%20Reference) (OtherComp :type Primitive%20Component%20Object%20Reference) (OtherBodyIndex :type Integer) (bFromSweep :type Boolean) (SweepResult :type Hit%20Result%20Structure%20%28by%20ref%29))
  ;[0.2 1 0.6] Component Overlap BP_DissappearingItem w/ FOV (MARK)
  (bind _asbp_disappearing_item (Utilities|Casting|CastToBP_DisappearingItem OtherActor))
  (Variables|/Game/Coding/MarkSanders/BP_DisappearingItem.BP_DisappearingItem_C|SetIsNotVisible _asbp_disappearing_item false)
  (Variables|/Game/Coding/MarkSanders/BP_DisappearingItem.BP_DisappearingItem_C|SetLookedAt _asbp_disappearing_item true))

(event OnComponentEndOverlap(FOV)
  (params (OverlappedComponent :type Primitive%20Component%20Object%20Reference) (OtherActor :type Actor%20Object%20Reference) (OtherComp :type Primitive%20Component%20Object%20Reference) (OtherBodyIndex :type Integer))
  ;[0.2 1 0.6] Component Overlap BP_DissappearingItem w/ FOV (MARK)
  (bind _asbp_disappearing_item (Utilities|Casting|CastToBP_DisappearingItem OtherActor))
  (Variables|/Game/Coding/MarkSanders/BP_DisappearingItem.BP_DisappearingItem_C|SetIsNotVisible _asbp_disappearing_item true))

(event OnComponentBeginOverlap(CapsuleComponent)
  (params (OverlappedComponent :type Primitive%20Component%20Object%20Reference) (OtherActor :type Actor%20Object%20Reference) (OtherComp :type Primitive%20Component%20Object%20Reference) (OtherBodyIndex :type Integer) (bFromSweep :type Boolean) (SweepResult :type Hit%20Result%20Structure%20%28by%20ref%29))
  ;[0.2 1 0.6] Component Overlap BP_DissappearingItem w/ FOV (MARK)
  (bind _asbp_disappearing_item (Utilities|Casting|CastToBP_DisappearingItem OtherActor))
  (Variables|/Game/Coding/MarkSanders/BP_DisappearingItem.BP_DisappearingItem_C|SetInTheRoom _asbp_disappearing_item true))

(event OnComponentEndOverlap(CapsuleComponent)
  (params (OverlappedComponent :type Primitive%20Component%20Object%20Reference) (OtherActor :type Actor%20Object%20Reference) (OtherComp :type Primitive%20Component%20Object%20Reference) (OtherBodyIndex :type Integer))
  ;[0.2 1 0.6] Component Overlap BP_DissappearingItem w/ FOV (MARK)
  (bind _asbp_disappearing_item (Utilities|Casting|CastToBP_DisappearingItem OtherActor))
  (Variables|/Game/Coding/MarkSanders/BP_DisappearingItem.BP_DisappearingItem_C|SetInTheRoom _asbp_disappearing_item false))

(event Custom|ResumePressed
  (bind _returnvalue (Game|GetPlayerController 0))
  (bind _pausemenu (Variables|Default|GetPauseMenu))
  ;[1 0.3968 0.7011] Open Pause Menu (Keagon)
  (Development|PrintString "CharacterResumePressed")
  (if (Variables|Default|GetPauseOpen)
    (Variables|Default|SetPauseOpen false)
    (Widget|RemovefromParent _pausemenu)
    (if (not (Variables|Default|GetMenuOpen))
      (Game|SetGamePaused false)
      (Input|SetInputModeGameOnly _returnvalue false)
      (Variables|/Script/Engine.PlayerController|SetbShowMouseCursor _returnvalue false)
      (else
        (Variables|/Script/Engine.PlayerController|SetbShowMouseCursor _returnvalue true :!label _label)))
    (else
      (Variables|Default|SetPauseOpen true)
      (UserInterface|Viewport|AddtoViewport _pausemenu 0)
      (Game|SetGamePaused true)
      (Input|SetInputModeGameandUI _returnvalue _pausemenu "DoNotLock" false false)
      (goto _label))))

(event Custom|Gameplay%20Start
  ;[1 0.3968 0.7011] Set Crosshair Visible (Keagon)
  (Class|Image|SetOpacity (Variables|/Game/Coding/KeagonTaylor/Blueprints/W_Crosshair.W_Crosshair_C|GetCrosshair_Dot (Variables|Default|GetCrosshair)) 0.75))

(event Input|EnhancedActionEvents|EnhancedInputActionIA_OpenPause
  (params (ActionValue :type Boolean) (ElapsedSeconds :type Float%20%28double-precision%29) (TriggeredSeconds :type Float%20%28double-precision%29) (InputAction :type Input%20Action%20Object%20Reference :default "/Game/Coding/KeagonTaylor/Inputs/InputMaps/IA_OpenPause.IA_OpenPause"))
  (bind _returnvalue (Game|GetPlayerController 0))
  (bind _pausemenu (Variables|Default|GetPauseMenu))
  ;[1 0.3968 0.7011] Open Pause Menu (Keagon)
  (:Started
    (if (Variables|Default|GetProcessing) :!label _label
      (Utilities|FlowControl|Delay 0.5)
      (goto _label)
      (else
        (if (Variables|Default|GetSaveDisabled)
          (Development|PrintText "Save Disabled"))
        (if (Variables|Default|GetPauseOpen)
          (Variables|Default|SetPauseOpen false)
          (Widget|RemovefromParent _pausemenu)
          (if (not (Variables|Default|GetMenuOpen))
            (Game|SetGamePaused false)
            (Input|SetInputModeGameOnly _returnvalue false)
            (Variables|/Script/Engine.PlayerController|SetbShowMouseCursor _returnvalue false)
            (else
              (Variables|/Script/Engine.PlayerController|SetbShowMouseCursor _returnvalue true :!label _label_2)))
          (else
            (Variables|Default|SetPauseOpen true)
            (UserInterface|Viewport|AddtoViewport _pausemenu 0)
            (Game|SetGamePaused true)
            (Input|SetInputModeGameandUI _returnvalue _pausemenu "DoNotLock" false false)
            (goto _label_2)))))))

(event Input|EnhancedActionEvents|EnhancedInputActionIA_OpenMenu
  (params (ActionValue :type Boolean) (ElapsedSeconds :type Float%20%28double-precision%29) (TriggeredSeconds :type Float%20%28double-precision%29) (InputAction :type Input%20Action%20Object%20Reference :default "/Game/Coding/KeagonTaylor/Inputs/InputMaps/IA_OpenMenu.IA_OpenMenu"))
  (bind _returnvalue (Game|GetPlayerController 0))
  (bind _menu (Variables|Default|GetMenu))
  (bind (_sizex _sizey) (HUD|GetViewportSize _returnvalue))
  ;[1 0.3961 0.702] Opening Menu (Keagon)
  (:Started
    (Variables|Default|SetWidgetID 0)
    (if (not (Variables|Default|GetProcessing))
      (Variables|Default|SetProcessing true)
      (if (Variables|Default|GetMenuOpen)
        (Variables|/Script/Engine.PlayerController|SetbShowMouseCursor _returnvalue false)
        (Input|SetInputModeGameOnly _returnvalue false)
        (Widget|SetVisibility _menu "Hidden")
        (Game|SetGamePaused false)
        (Utilities|FlowControl|Delay (Variables|Default|GetCloseDelay))
        (Variables|Default|SetMenuOpen false)
        (Variables|Default|SetProcessing false)
        (Class|Image|SetOpacity (Variables|/Game/Coding/KeagonTaylor/Blueprints/W_Crosshair.W_Crosshair_C|GetCrosshair_Dot (Variables|Default|GetCrosshair)) 0.75)
        (else
          (Class|Image|SetOpacity (Variables|/Game/Coding/KeagonTaylor/Blueprints/W_Crosshair.W_Crosshair_C|GetCrosshair_Dot (Variables|Default|GetCrosshair)) 0.0)
          (Variables|Default|SetMenuOpen true)
          (Utilities|FlowControl|Delay (Variables|Default|GetOpenDelay))
          (Game|SetGamePaused true)
          (Class|WidgetSwitcher|SetActiveWidgetIndex (Variables|/Game/Coding/KeagonTaylor/Blueprints/Menus/WP_Menu.WP_Menu_C|GetWidgetSwitcher _menu) (Variables|Default|GetWidgetID))
          (Widget|SetVisibility _menu "Visible")
          (Variables|/Script/Engine.PlayerController|SetbShowMouseCursor _returnvalue true)
          (Class|PlayerController|SetMouseLocation _returnvalue (/ _sizex 2) (/ _sizey 2))
          (Input|SetInputModeGameandUI _returnvalue _menu "DoNotLock" true false)
          (Variables|Default|SetProcessing false))))))

(event Input|EnhancedActionEvents|EnhancedInputActionIA_OpenMap
  (params (ActionValue :type Boolean) (ElapsedSeconds :type Float%20%28double-precision%29) (TriggeredSeconds :type Float%20%28double-precision%29) (InputAction :type Input%20Action%20Object%20Reference :default "/Game/Coding/KeagonTaylor/Inputs/InputMaps/IA_OpenMap.IA_OpenMap"))
  (bind _returnvalue (Game|GetPlayerController 0))
  (bind _menu (Variables|Default|GetMenu))
  (bind (_sizex _sizey) (HUD|GetViewportSize _returnvalue))
  ;[1 0.3961 0.702] Opening Menu (Keagon)
  (:Started
    (Variables|Default|SetWidgetID 1)
    (if (not (Variables|Default|GetProcessing))
      (Variables|Default|SetProcessing true)
      (if (Variables|Default|GetMenuOpen)
        (Variables|/Script/Engine.PlayerController|SetbShowMouseCursor _returnvalue false)
        (Input|SetInputModeGameOnly _returnvalue false)
        (Widget|SetVisibility _menu "Hidden")
        (Game|SetGamePaused false)
        (Utilities|FlowControl|Delay (Variables|Default|GetCloseDelay))
        (Variables|Default|SetMenuOpen false)
        (Variables|Default|SetProcessing false)
        (Class|Image|SetOpacity (Variables|/Game/Coding/KeagonTaylor/Blueprints/W_Crosshair.W_Crosshair_C|GetCrosshair_Dot (Variables|Default|GetCrosshair)) 0.75)
        (else
          (Class|Image|SetOpacity (Variables|/Game/Coding/KeagonTaylor/Blueprints/W_Crosshair.W_Crosshair_C|GetCrosshair_Dot (Variables|Default|GetCrosshair)) 0.0)
          (Variables|Default|SetMenuOpen true)
          (Utilities|FlowControl|Delay (Variables|Default|GetOpenDelay))
          (Game|SetGamePaused true)
          (Class|WidgetSwitcher|SetActiveWidgetIndex (Variables|/Game/Coding/KeagonTaylor/Blueprints/Menus/WP_Menu.WP_Menu_C|GetWidgetSwitcher _menu) (Variables|Default|GetWidgetID))
          (Widget|SetVisibility _menu "Visible")
          (Variables|/Script/Engine.PlayerController|SetbShowMouseCursor _returnvalue true)
          (Class|PlayerController|SetMouseLocation _returnvalue (/ _sizex 2) (/ _sizey 2))
          (Input|SetInputModeGameandUI _returnvalue _menu "DoNotLock" true false)
          (Variables|Default|SetProcessing false))))))

(event Input|EnhancedActionEvents|EnhancedInputActionIA_OpenSettings
  (params (ActionValue :type Boolean) (ElapsedSeconds :type Float%20%28double-precision%29) (TriggeredSeconds :type Float%20%28double-precision%29) (InputAction :type Input%20Action%20Object%20Reference :default "/Game/Coding/KeagonTaylor/Inputs/InputMaps/IA_OpenSettings.IA_OpenSettings"))
  (bind _returnvalue (Game|GetPlayerController 0))
  (bind _menu (Variables|Default|GetMenu))
  (bind (_sizex _sizey) (HUD|GetViewportSize _returnvalue))
  ;[1 0.3961 0.702] Opening Menu (Keagon)
  (:Started
    (Variables|Default|SetWidgetID 2)
    (if (not (Variables|Default|GetProcessing))
      (Variables|Default|SetProcessing true)
      (if (Variables|Default|GetMenuOpen)
        (Variables|/Script/Engine.PlayerController|SetbShowMouseCursor _returnvalue false)
        (Input|SetInputModeGameOnly _returnvalue false)
        (Widget|SetVisibility _menu "Hidden")
        (Game|SetGamePaused false)
        (Utilities|FlowControl|Delay (Variables|Default|GetCloseDelay))
        (Variables|Default|SetMenuOpen false)
        (Variables|Default|SetProcessing false)
        (Class|Image|SetOpacity (Variables|/Game/Coding/KeagonTaylor/Blueprints/W_Crosshair.W_Crosshair_C|GetCrosshair_Dot (Variables|Default|GetCrosshair)) 0.75)
        (else
          (Class|Image|SetOpacity (Variables|/Game/Coding/KeagonTaylor/Blueprints/W_Crosshair.W_Crosshair_C|GetCrosshair_Dot (Variables|Default|GetCrosshair)) 0.0)
          (Variables|Default|SetMenuOpen true)
          (Utilities|FlowControl|Delay (Variables|Default|GetOpenDelay))
          (Game|SetGamePaused true)
          (Class|WidgetSwitcher|SetActiveWidgetIndex (Variables|/Game/Coding/KeagonTaylor/Blueprints/Menus/WP_Menu.WP_Menu_C|GetWidgetSwitcher _menu) (Variables|Default|GetWidgetID))
          (Widget|SetVisibility _menu "Visible")
          (Variables|/Script/Engine.PlayerController|SetbShowMouseCursor _returnvalue true)
          (Class|PlayerController|SetMouseLocation _returnvalue (/ _sizex 2) (/ _sizey 2))
          (Input|SetInputModeGameandUI _returnvalue _menu "DoNotLock" true false)
          (Variables|Default|SetProcessing false))))))

(event EventTick
  (params (DeltaSeconds :type Float%20%28single-precision%29))
  (bind _returnvalue (Game|GetPlayerCameraManager 0))
  (bind _charactermovement (Variables|Character|GetCharacterMovement))
  (bind _returnvalue_2 (Transformation|GetActorLocation _returnvalue))
  ;[0.3 1 0.3] gravity off and on (gravity included!) Ace
  (if (Variables|Default|Getgravity)
    (if (Variables|Default|GetSlam?)
      (Physics|AddImpulse (Variables|Character|GetCharacterMovement) "0.000000,0.000000,-10000.000000" false)
      (Variables|Default|SetSlam? false))
    (Variables|/Script/Engine.CharacterMovementComponent|SetMaxWalkSpeed _charactermovement 4e+02)
    (elif (Variables|Default|GetGeneratorRoom?Player)
      (Variables|Default|SetSlam? true)
      (Variables|/Script/Engine.CharacterMovementComponent|SetMaxWalkSpeed _charactermovement 1e+02)
      (Physics|AddForce (Variables|Character|GetCharacterMovement) "0.000000,0.000000,99000.000000")
      (else
        (Utilities|FlowControl|FlipFlop
          (:A
            (Variables|/Script/Engine.CharacterMovementComponent|SetMaxWalkSpeed (Variables|Character|GetCharacterMovement) 1e+02)
            (Variables|Default|SetSlam? false)
            (Physics|AddForce (Variables|Character|GetCharacterMovement) "0.000000,0.000000,98000.000000"))
          (:B
            (Variables|/Script/Engine.CharacterMovementComponent|SetMaxWalkSpeed (Variables|Character|GetCharacterMovement) 1e+02)
            (Variables|Default|SetSlam? false)
            (Physics|AddForce (Variables|Character|GetCharacterMovement) "0.000000,0.000000,97600.000000"))))))
  ;[0 0.3294 1] Interact (Luke)
  (bind (_outhit _returnvalue_3) (Collision|LineTraceByChannel _returnvalue_2 (+ (* (Transformation|GetActorForwardVector _returnvalue) (Variables|Default|GetDistanceForwardLook)) _returnvalue_2) "TraceTypeQuery1" false 0 "None"))
  (if _returnvalue_3
    (Variables|Default|SetObjLookedAt (.HitActor (Collision|BreakHitResult _outhit)))
    (else
      (Variables|Default|SetObjLookedAt 0))))

(event Collision|EventActorBeginOverlap
  (params (OtherActor :type Actor%20Object%20Reference))
  ;[0 0.3278 1] Save N' Load (Luke)
  (if (== (Utilities|GetClass OtherActor) "/Game/Coding/Luke_Samuelson/SaveSystem/BP_Savepoint.BP_Savepoint_C")
    (bind _asbp_game_variables (Utilities|Casting|CastToBP_GameVariables (Game|GetGameInstance)))
    (Default|Save _asbp_game_variables)
    (Development|PrintString "Save")))

(event Input|ActionEvents|InputActionInteract
  (params (Key :type Key%20Structure :default "None"))
  ;[0 0.3294 1] Interact (Luke)
  (:Pressed
    (bind _asbp_master_interact (Utilities|Casting|CastToBP_MasterInteract (Variables|Default|GetObjLookedAt)))
    (Default|InteractwithObject _asbp_master_interact)))

(event Input|AxisEvents|InputAxisForwardBack
  (params (AxisValue :type Float%20%28single-precision%29))
  ;[0.3 1 0.3] WASD Movement (Ace)
  (if (Variables|Default|GetWASD%20Movement)
    (Pawn|Input|AddMovementInput (Transformation|GetActorForwardVector) (/ AxisValue 1.25) false)))

(event Input|AxisEvents|InputAxisLeftRight
  (params (AxisValue :type Float%20%28single-precision%29))
  ;[0.3 1 0.3] WASD Movement (Ace)
  (if (Variables|Default|GetWASD%20Movement)
    (Pawn|Input|AddMovementInput (Transformation|GetActorRightVector) (/ AxisValue 1.25) false)))

(event Input|AxisEvents|InputAxisCameraY
  (params (AxisValue :type Float%20%28single-precision%29))
  ;[0.3 1 0.3] Camera (Ace)
  (Utilities|IsMenuClosed
    (:then
      (Pawn|Input|AddControllerPitchInput (* AxisValue (Variables|Default|GetCamYInvertVal) (Variables|Default|GetCamSensitivity))))))

(event Input|AxisEvents|InputAxisCameraX
  (params (AxisValue :type Float%20%28single-precision%29))
  ;[0.3 1 0.3] Camera (Ace)
  (Utilities|IsMenuClosed
    (:then
      (Pawn|Input|AddControllerYawInput (* AxisValue (Variables|Default|GetCamSensitivity))))))

(event Input|KeyboardEvents|E
  (params (Key :type Key%20Structure :default "None"))
  (bind _camera1 (Variables|Camera|GetCamera1))
  (bind _returnvalue (Transformation|GetWorldLocation _camera1))
  ;[1 1 1] Handle Movement (Derek)
  (:Pressed
    (bind _outhit (Collision|LineTraceByChannel _returnvalue (+ _returnvalue (* (Math|Vector|GetForwardVector (Transformation|GetWorldRotation _camera1)) 1.5e+03)) "TraceTypeQuery1" false 0 "None"))
    (if (.bBlockingHit (Collision|BreakHitResult _outhit))
      (Utilities|String|LogString "Hit")
      (bind _asbp_handle (Utilities|Casting|CastToBP_handle (.HitActor (Collision|BreakHitResult _outhit))))
      (Development|PrintString (Utilities|GetDisplayName (.HitActor (Collision|BreakHitResult _outhit))))
      (Default|GotoHandle _asbp_handle))))

(event Input|KeyboardEvents|LeftCtrl
  (params (Key :type Key%20Structure :default "None"))
  ;[0.3 1 0.3] Crouch (Ace)
  (:Pressed
    (Character|Crouch)
    ;[0 0.3278 1] Make Player Invisible
    (bind _asbp_player_character_ace (Utilities|Casting|CastToBP_PlayerCharacterACE (Game|GetPlayerCharacter 0)))
    (Rendering|SetVisibility (Variables|/Script/Engine.Character|GetMesh _asbp_player_character_ace) false false))
  (:Released
    (Character|UnCrouch)
    (bind _asbp_player_character_ace_2 (Utilities|Casting|CastToBP_PlayerCharacterACE (Game|GetPlayerCharacter 0)))
    (Rendering|SetVisibility (Variables|/Script/Engine.Character|GetMesh _asbp_player_character_ace_2) true false)))

(event Input|KeyboardEvents|1
  (params (Key :type Key%20Structure :default "None"))
  (bind _returnvalue (Game|GetPlayerController 0))
  (bind _returnvalue_2 (Game|GetPlayerController 0))
  ;[0.3 1 0.3] Sensitivity Slider widgets menu, to be implemented into final settings menu. Also CamYInvert at the end (Ace)
  (:Pressed
    (if (Game|IsGamePaused)
      (Game|SetGamePaused false)
      (Widget|RemovefromParent (stale _returnvalue_3))
      (Input|SetInputModeGameOnly _returnvalue false)
      (Variables|/Script/Engine.PlayerController|SetbShowMouseCursor _returnvalue false)
      (CallFunction|SetYInvert)
      (else
        (Game|SetGamePaused true)
        (bind _returnvalue_3 (UserInterface|CreateWidget "/Game/Coding/AceWest/BP_AceMenu.BP_AceMenu_C"))
        (UserInterface|Viewport|AddtoViewport _returnvalue_3 0)
        (Input|SetInputModeGameandUI _returnvalue_2 0 "DoNotLock" false false)
        (Variables|/Script/Engine.PlayerController|SetbShowMouseCursor _returnvalue_2 true)
        (CallFunction|SetYInvert)))))

(event Input|KeyboardEvents|T
  (params (Key :type Key%20Structure :default "None"))
  ;[0 0.3278 1] Save N' Load (Luke)
  (:Pressed
    (bind _asbp_game_variables (Utilities|Casting|CastToBP_GameVariables (Game|GetGameInstance)))
    (Default|Load _asbp_game_variables)
    (Development|PrintString "Load")))

(event Input|KeyboardEvents|SpaceBar
  (params (Key :type Key%20Structure :default "None"))
  ;[0.3 1 0.3] Jump (Ace)
  (:Pressed
    (Character|Jump)))

(fn ConstructionScript)

(fn SetYInvert
  (if (Variables|Default|GetCamYInvert)
    (Variables|Default|SetCamYInvertVal -1)
    (else
      (Variables|Default|SetCamYInvertVal 1))))

(fn AddItem
  (params (ItemName :type Text) (ItemDescription :type Text) (ItemImage :type Slate%20Brush%20Structure))
  ;[1 0.3968 0.7011] Add Item (Keagon)
  (Default|AddItem (Variables|Default|GetBPC_Inventory) ItemName ItemDescription)
  (Default|AddItem (Variables|Default|GetMenu) ItemImage (Utilities|Array|LastIndex (Variables|/Game/Coding/KeagonTaylor/Blueprints/Menus/InventoryWidgets/BPC_Inventory.BPC_Inventory_C|GetItemNameArray (Variables|Default|GetBPC_Inventory)))))

(fn SwapItem
  (bind _bpc_inventory (Variables|Default|GetBPC_Inventory))
  (bind _itemnamearray (Variables|/Game/Coding/KeagonTaylor/Blueprints/Menus/InventoryWidgets/BPC_Inventory.BPC_Inventory_C|GetItemNameArray _bpc_inventory))
  (bind _output (Utilities|Array|Get(acopy) _itemnamearray))
  ;[1 0.3968 0.7011] Swap Item (Keagon)
  (Development|PrintText _output)
  (Default|SwapItem (Variables|Default|GetMenu) _output (Utilities|Array|Get(acopy) (Variables|/Game/Coding/KeagonTaylor/Blueprints/Menus/InventoryWidgets/BPC_Inventory.BPC_Inventory_C|GetItemDescriptionArray _bpc_inventory))))

(fn CreateCrosshair
  (bind _returnvalue (Game|GetPlayerController 0))
  (bind _returnvalue_2 (PlayerController|LocalPlayerSubsystems|GetEnhancedInputLocalPlayerSubsystem _returnvalue))
  (Utilities|FlowControl|Sequence
    (:then_0
      (bind _returnvalue_3 (UserInterface|CreateWidget "/Game/Coding/KeagonTaylor/Blueprints/W_Crosshair.W_Crosshair_C"))
      (bind _output_get (Variables|Default|SetCrosshair _returnvalue_3))
      (UserInterface|Viewport|AddtoViewport _output_get 0)
      (Widget|SetRenderOpacity _output_get 0.75)
      (Utilities|IsValid _returnvalue_2
        (:Is%20Valid
          (Input|AddMappingContext _returnvalue_2 "/Game/Coding/KeagonTaylor/Inputs/IMC_Basic.IMC_Basic" 0 "(bIgnoreAllPressedKeysUntilRelease=True,bForceImmediately=False)")
          (bind _returnvalue_4 (UserInterface|CreateWidget "/Game/Coding/KeagonTaylor/Blueprints/Menus/WP_Menu.WP_Menu_C"))
          (bind _output_get_2 (Variables|Default|SetMenu _returnvalue_4))
          (UserInterface|Viewport|AddtoViewport _output_get_2 0)
          (Widget|SetVisibility _output_get_2 "Hidden")
          (Input|EnableInput _returnvalue)
          (Variables|Default|SetOpenDelay 1.0)
          (Variables|Default|SetMenuOpen false)
          (Variables|Default|SetCloseDelay 0.5))))
    (:then_1
      (bind _returnvalue_5 (UserInterface|CreateWidget "/Game/Coding/KeagonTaylor/Blueprints/Menus/WP_Tasks.WP_Tasks_C"))
      (Variables|Default|SetTasksMenu _returnvalue_5)
      (bind _returnvalue_6 (UserInterface|CreateWidget "/Game/Coding/KeagonTaylor/Blueprints/Menus/W_PauseMenu.W_PauseMenu_C"))
      (Variables|Default|SetPauseMenu _returnvalue_6))
    (:then_2
      (bind _returnvalue_7 (UserInterface|CreateWidget "/Game/Coding/Luke_Samuelson/Widgets/W_Alpha.W_Alpha_C"))
      (UserInterface|Viewport|AddtoViewport _returnvalue_7 0))))